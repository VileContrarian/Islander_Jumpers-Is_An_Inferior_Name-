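; BP_FireColoured is a coloured fire prop actor that turns to face the player camera like a billboard.
; On BeginPlay it starts Light_flicker and a looping timer that calls GetAngle ten times a second.
; GetAngle flattens the direction to the camera onto the horizontal plane and sets it as the actor's rotation, so the fire stays upright without using Tick.
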(event EventBeginPlay
  (Utilities|Time|SetTimerbyFunctionName 0 "getAngle" 0.1 true)
  (Timeline|light_flicker Play))

(fn ConstructionScript)

(fn GetAngle
  (Transformation|SetActorRotation (Math|Conversions|RotationFromXVector (Math|Vector|Normalize (* (- (Camera|GetCameraLocation (Game|GetPlayerCameraManager 0)) (Transformation|GetActorLocation)) "1.000000,1.000000, 0")))))
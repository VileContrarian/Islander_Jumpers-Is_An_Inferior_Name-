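; Chevron prop Blueprint that bobs its front plane vertically and pulses its glow.
; Construction creates dynamic materials for both planes, though only the front one is animated.
; A looping timer at about 30 fps, used instead of Tick, advances a wrapping manual clock by Frequency.
; That clock's sine sets the front plane's height and its material's clamped Intensity and AlphaMultiplier parameters.
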(event EventBeginPlay
  ;[1 1 1] 30 fps
  (Utilities|Time|SetTimerbyFunctionName 0 "TimedLoop" 0.033 true))

(fn ConstructionScript
  (bind _returnvalue (Rendering|Material|CreateDynamicMaterialInstance (Variables|Default|GetFrontPlane) 0 "/Game/Materials/SpeedBooster/M_Chevron1.M_Chevron1" "None" :!class /Script/Engine.PrimitiveComponent))
  (Variables|Default|SetFrontMat _returnvalue)
  (bind _returnvalue_2 (Rendering|Material|CreateDynamicMaterialInstance (Variables|Default|GetBackPlane) 0 "/Game/Materials/SpeedBooster/M_Chevron2.M_Chevron2" "None" :!class /Script/Engine.PrimitiveComponent))
  (Variables|Default|SetBackMat _returnvalue_2))

(fn Animate
  (params (Period :type Float%20%28single-precision%29%20%28by%20ref%29))
  (Transformation|SetRelativeLocation (Variables|Default|GetFrontPlane) (Math|Vector|MakeVector 0.0 0.0 (* (Math|Trig|Sin(Radians) Period) (Variables|Default|GetAmplitude))) false false))

(fn TimedLoop
  (bind _period (CallFunction|ManualClock))
  (CallFunction|Animate _period)
  (CallFunction|GlowingFX _period))

(fn GlowingFX
  (params (Period :type Float%20%28single-precision%29%20%28by%20ref%29))
  (bind _returnvalue (Math|Trig|Sin(Radians) Period))
  (bind _frontmat (Variables|Default|GetFrontMat))
  (bind _intensityamplitude (Variables|Default|GetIntensityAmplitude))
  (bind _returnvalue_2 (* _returnvalue _intensityamplitude))
  (bind _returnvalue_3 (Math|Float|Clamp(Float) _returnvalue_2 5.0 _intensityamplitude))
  (Rendering|Material|SetScalarParameterValue _frontmat "Intensity" _returnvalue_3 :!class /Script/Engine.MaterialInstanceDynamic)
  (Rendering|Material|SetScalarParameterValue _frontmat "AlphaMultiplier" (Math|Float|Clamp(Float) _returnvalue_3 0.5) :!class /Script/Engine.MaterialInstanceDynamic))

(fn ManualClock
  ;[1 1 1] Manual Clock Cycle
  (bind _output_get (Variables|Default|SetTimer (+ (stale _output_get) (Variables|Default|GetFrequency))))
  (if (> _output_get 1e+02)
    ;[1 1 1] Resetting Clock
    (Variables|Default|SetTimer 0.0))
  (return (Variables|Default|GetTimer)))
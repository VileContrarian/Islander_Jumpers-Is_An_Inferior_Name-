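; Scene component for a hovering vehicle that applies levitation force to a car mesh supplied through InitComponent.
; Each tick it traces along its down vector, records ground contact and, while the mesh moves downward, pushes along the hit normal, fading with distance.
; Angular damping is set alongside the push to reduce wobble.
; An experimental Jump applies a large normal-aligned force, temporarily lowering mass around the call.
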(event Custom|InitComponent
  (params (StaticMesh :type Static%20Mesh%20Component%20Object%20Reference))
  (Variables|Default|SetCarMesh StaticMesh))

(event EventBeginPlay)

(event EventTick
  (params (DeltaSeconds :type Float%20%28single-precision%29))
  (bind _returnvalue (Transformation|GetWorldLocation))
  (bind _carmesh (Variables|Default|GetCarMesh))
  ;[1 1 1] Raycast
  (bind (_outhit _returnvalue_2) (Collision|LineTraceByChannel _returnvalue (+ _returnvalue (* (* (Math|Vector|GetUpVector) -1.0) (Variables|Default|GetTraceLength))) "TraceTypeQuery1" false 0 "ForOneFrame"))
  (if _returnvalue_2
    ;[1 1 1] Check if on the air
    (Variables|Default|SetisHitGround true)
    (else
      (Variables|Default|SetisHitGround false)))
  ;[1 1 1] Only Levitate if near ground AND 'falling'
  (bind _returnvalue_3 (Physics|GetPhysicsLinearVelocity (Variables|Default|GetCarMesh) "None"))
  (if (< (.z _returnvalue_3) 0.0)
    ;[1 1 1] Force to Levitate
    (Class|PrimitiveComponent|AddForceatLocation _carmesh (* (.ImpactNormal (Collision|BreakHitResult _outhit)) (Math|Float|Lerp (* (Variables|Default|GetHoverForce) 1e+04) 0.0 (/ (Math|Vector|VectorLength (- (Transformation|GetWorldLocation) (.Location (Collision|BreakHitResult _outhit)))) (Variables|Default|GetTraceLength)))) (Transformation|GetWorldLocation) "None")
    ;[1 1 1] Reduce the "wobbling" of the vehicle
    (Class|PrimitiveComponent|SetAngularDamping _carmesh (Variables|Default|GetAngularDamping))))

(fn Jump
  (bind _returnvalue (Transformation|GetWorldLocation))
  (bind _carmesh (Variables|Default|GetCarMesh))
  ;[1 1 1] Experimental for now
  (bind _outhit (Collision|LineTraceByChannel _returnvalue (+ _returnvalue (* (* (Math|Vector|GetUpVector) -1.0) (Variables|Default|GetTraceLength))) "TraceTypeQuery1" false 0 "ForOneFrame"))
  (if (.bBlockingHit (Collision|BreakHitResult _outhit))
    (Class|PrimitiveComponent|SetMassOverrideinKg _carmesh "None" 1.0 true)
    (Class|PrimitiveComponent|AddForceatLocation _carmesh (* (.ImpactNormal (Collision|BreakHitResult _outhit)) 5e+06) (Transformation|GetWorldLocation) "None")
    (Class|PrimitiveComponent|SetMassOverrideinKg _carmesh "None" 1e+02 true)))
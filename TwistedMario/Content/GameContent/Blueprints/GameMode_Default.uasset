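; Default game mode that spawns a BP_VehicleTypeB vehicle for each player joining the game.
; On PostLogin, the server waits briefly to avoid networking collisions, stores the player controller, then spawns the vehicle at the player start named by a prefix plus PlayerIndex.
; PlayerIndex has zero added on each login, so this graph never advances it, and the manual Possess call is disconnected and never runs.
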(event EventBeginPlay)

(event EventTick
  (params (DeltaSeconds :type Float%20%28single-precision%29)))

(event EventPostLogin
  (params (NewPlayer :type Player%20Controller%20Object%20Reference))
  ;[1 1 1] Gives Player A Controller When Joining Game
  ;;[1 1 1] Adds Delay to Prevent Networking Collision
  (Networking|SwitchHasAuthority
    (:Authority
      (Utilities|FlowControl|Delay 0.2)
      (Variables|Default|SetPlayerIndex (+ (Variables|Default|GetPlayerIndex) 0))
      ;;[1 1 1] Casting To Player Controller just in Case
      (bind _asplayer_controller (Utilities|Casting|CastToPlayerController NewPlayer))
      (Variables|Default|SetPlayerControllerRef _asplayer_controller)
      ;;[1 1 1] Spawns Vehicle On To Map
      (Game|SpawnActorfromClass "/Game/GameContent/Blueprints/VehicleBase/BP_VehicleTypeB.BP_VehicleTypeB_C" (Transformation|GetActorTransform (Class|GameModeBase|FindPlayerStart (Variables|Default|GetPlayerControllerRef) (Utilities|String|Append (Variables|Default|GetPlayerSpawnPointName) (Utilities|String|ToString(Integer) (Variables|Default|GetPlayerIndex))))) "AlwaysSpawn" (Game|GetGameMode) 0))))

(fn ConstructionScript)
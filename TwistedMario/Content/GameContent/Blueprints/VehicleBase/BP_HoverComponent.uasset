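; Scene component for a hover vehicle that applies a levitation force to the car mesh supplied through InitComponent.
; Each tick it line-traces along its down vector and records whether ground is hit.
; While the mesh moves downward, it pushes along the impact normal at the component's location, fading force with distance, and sets angular damping to reduce wobble.
; A Timer-based fixed-interval trace gate is left disconnected.
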(event Custom|InitComponent
  (params (StaticMesh :type Static%20Mesh%20Component%20Object%20Reference))
  (bind _output_get (Variables|Default|SetCarMesh StaticMesh))
  (Variables|Default|SetMass (Physics|GetMass _output_get)))

(event EventBeginPlay)

(event EventTick
  (params (DeltaSeconds :type Float%20%28single-precision%29))
  (bind _returnvalue (Transformation|GetWorldLocation))
  (bind _carmesh (Variables|Default|GetCarMesh))
  ;[1 1 1] Raycast
  (bind (_outhit _returnvalue_2) (Collision|LineTraceByChannel _returnvalue (+ _returnvalue (* (* (Math|Vector|GetUpVector) -1.0) (Variables|Default|GetTraceLength))) "TraceTypeQuery1" false 0 "ForOneFrame"))
  (if _returnvalue_2
    ;[1 1 1] Check if on the air
    (Variables|Default|SetisHitGround true)
    (else
      (Variables|Default|SetisHitGround false)))
  ;[1 1 1] Hover when falling close to the ground
  (bind _returnvalue_3 (Physics|GetPhysicsLinearVelocity (Variables|Default|GetCarMesh) "None"))
  (if (< (.z _returnvalue_3) 0.0)
    (bind _output_get (Variables|Default|SetImpactLocation (.ImpactNormal (Collision|BreakHitResult _outhit))))
    (Variables|Default|SetPrevForce (Math|Float|Lerp (* 1e+04 (Variables|Default|GetHoverForce)) 0.0 (/ (Math|Vector|VectorLength (- (Transformation|GetWorldLocation) (.Location (Collision|BreakHitResult _outhit)))) (Variables|Default|GetTraceLength))))
    ;[1 1 1] Force to Levitate
    (Class|PrimitiveComponent|AddForceatLocation _carmesh (* _output_get (Math|Float|Lerp (* 1e+04 (Variables|Default|GetHoverForce)) 0.0 (/ (Math|Vector|VectorLength (- (Transformation|GetWorldLocation) (.Location (Collision|BreakHitResult _outhit)))) (Variables|Default|GetTraceLength)))) (Transformation|GetWorldLocation self) "None")
    ;[1 1 1] Reduce the "wobbling" of the vehicle
    (Class|PrimitiveComponent|SetAngularDamping _carmesh (Variables|Default|GetAngularDamping))))

(fn Timer
  (params (DeltaTime :type Float%20%28single-precision%29))
  (bind _output_get (Variables|Default|SetElapsedTime (+ DeltaTime (Variables|Default|GetElapsedTime))))
  (if (> _output_get 1e+03)
    (Variables|Default|SetElapsedTime (- (Variables|Default|GetElapsedTime) 1e+03))
    (return (Variables|Default|GetElapsedTime))))
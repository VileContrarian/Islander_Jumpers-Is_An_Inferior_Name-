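; Base Blueprint for a hovering vehicle driven by a physics-simulated car body and four thruster components.
; Construction fetches the car mesh through GetCarMesh, enables physics and overrides the body's mass.
; BeginPlay initializes each thruster with the body, passes down shared hover force, trace length and angular damping, then sets the center of mass.
; Thruster4 is the exception, with its angular damping forced to zero.
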(event EventBeginPlay
  (CallFunction|InitThrusters)
  (Class|PrimitiveComponent|SetCenterOfMass (Variables|Default|GetCarBody) (Variables|Default|GetCenterOfMass) "None"))

(event Collision|EventActorBeginOverlap
  (params (OtherActor :type Actor%20Object%20Reference)))

(event EventTick
  (params (DeltaSeconds :type Float%20%28single-precision%29)))

(fn ConstructionScript
  (bind _carbody (Variables|Default|GetCarBody))
  (Class|VehicleBaseNoRoot|GetCarMesh _carbody)
  (Physics|SetSimulatePhysics _carbody true)
  (Class|PrimitiveComponent|SetMassOverrideinKg _carbody "None" (Variables|Default|Getmass) true))

(fn InitThrusters
  (bind _thruster2 (Variables|Default|GetThruster2))
  (bind _thruster4 (Variables|Default|GetThruster4))
  (bind _thruster1 (Variables|Default|GetThruster1))
  (bind _thruster3 (Variables|Default|GetThruster3))
  (Default|InitComponent _thruster3 (Variables|Default|GetCarBody))
  (Variables|/Game/GameContent/Blueprints/VehicleBase/BP_HoverComponent_SkeletalMesh.BP_HoverComponent_SkeletalMesh_C|SetHoverForce _thruster1 (Variables|Default|GetHoverForce))
  (Variables|/Game/GameContent/Blueprints/VehicleBase/BP_HoverComponent_SkeletalMesh.BP_HoverComponent_SkeletalMesh_C|SetHoverForce _thruster2 (Variables|Default|GetHoverForce))
  (Variables|/Game/GameContent/Blueprints/VehicleBase/BP_HoverComponent_SkeletalMesh.BP_HoverComponent_SkeletalMesh_C|SetHoverForce _thruster3 (Variables|Default|GetHoverForce))
  (Variables|/Game/GameContent/Blueprints/VehicleBase/BP_HoverComponent_SkeletalMesh.BP_HoverComponent_SkeletalMesh_C|SetHoverForce _thruster4 (Variables|Default|GetHoverForce))
  (Variables|/Game/GameContent/Blueprints/VehicleBase/BP_HoverComponent_SkeletalMesh.BP_HoverComponent_SkeletalMesh_C|SetTraceLength _thruster1 (Variables|Default|GetTraceLength))
  (Variables|/Game/GameContent/Blueprints/VehicleBase/BP_HoverComponent_SkeletalMesh.BP_HoverComponent_SkeletalMesh_C|SetTraceLength _thruster2 (Variables|Default|GetTraceLength))
  (Variables|/Game/GameContent/Blueprints/VehicleBase/BP_HoverComponent_SkeletalMesh.BP_HoverComponent_SkeletalMesh_C|SetTraceLength _thruster3 (Variables|Default|GetTraceLength))
  (Variables|/Game/GameContent/Blueprints/VehicleBase/BP_HoverComponent_SkeletalMesh.BP_HoverComponent_SkeletalMesh_C|SetTraceLength _thruster4 (Variables|Default|GetTraceLength))
  (Variables|/Game/GameContent/Blueprints/VehicleBase/BP_HoverComponent_SkeletalMesh.BP_HoverComponent_SkeletalMesh_C|SetAngularDamping _thruster1 (Variables|Default|GetAngularDamping))
  (Variables|/Game/GameContent/Blueprints/VehicleBase/BP_HoverComponent_SkeletalMesh.BP_HoverComponent_SkeletalMesh_C|SetAngularDamping _thruster2 (Variables|Default|GetAngularDamping))
  (Variables|/Game/GameContent/Blueprints/VehicleBase/BP_HoverComponent_SkeletalMesh.BP_HoverComponent_SkeletalMesh_C|SetAngularDamping _thruster3 (Variables|Default|GetAngularDamping))
  (Variables|/Game/GameContent/Blueprints/VehicleBase/BP_HoverComponent_SkeletalMesh.BP_HoverComponent_SkeletalMesh_C|SetAngularDamping _thruster4 0.0))
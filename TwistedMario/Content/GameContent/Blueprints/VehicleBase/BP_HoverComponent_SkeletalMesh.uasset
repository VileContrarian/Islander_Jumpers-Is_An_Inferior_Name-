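; Hover component for skeletal-mesh vehicles that levitates the car with a raycast spring-damper suspension.
; InitComponent receives the mesh, and a looping 0.01-second timer runs DoLevitation instead of Tick, aiming for similar physics across machines.
; Each call traces downward, updates the ground-hit flag, applies spring and damping force along the impact normal at the component's location, and sets angular damping to reduce wobble.
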(event Custom|InitComponent
  (params (SkeletalMesh :type Skeletal%20Mesh%20Component%20Object%20Reference))
  (bind _output_get (Variables|Default|SetCarMesh SkeletalMesh))
  (Variables|Default|SetMass (Physics|GetMass _output_get)))

(event EventBeginPlay
  ;[1 1 1 1 10] This is a timed loop that manually caps the call cycle of functions run within it. I'm using this to try to get all PC's to simulate similar physics behaviour regardless of their build, since UE doesn't have fixed Tick(). Methods called here are slower and maybe less accurate but generally have the same call rate in any system.
  (Utilities|Time|SetTimerbyFunctionName 0 "DoLevitation" 0.01 true))

(event EventTick
  (params (DeltaSeconds :type Float%20%28single-precision%29)))

(fn DoLevitation
  (bind _returnvalue (Transformation|GetWorldLocation))
  (bind _carmesh (Variables|Default|GetCarMesh))
  ;[1 1 1] Raycast
  (bind (_outhit _returnvalue_2) (Collision|LineTraceByChannel _returnvalue (+ _returnvalue (* (Math|Vector|GetUpVector) (* (Variables|Default|GetTraceLength) -1.0))) "TraceTypeQuery1" false 0 "None"))
  (if _returnvalue_2
    ;[1 1 1] Check if on the air
    (Variables|Default|SetisHitGround true)
    (else
      (Variables|Default|SetisHitGround false)))
  (bind _output_get (Variables|Default|SetDistanceHit (- (Variables|Default|GetTraceLength) (.Distance (Collision|BreakHitResult _outhit)))))
  ;[1 1 1] Force to Levitate
  (Class|PrimitiveComponent|AddForceatLocation _carmesh (* (.ImpactNormal (Collision|BreakHitResult _outhit)) (+ (* (/ (- _output_get (Variables|Default|GetPrevHit)) (Utilities|Time|GetWorldDeltaSeconds)) (Variables|Default|GetDampingCoeff)) (* _output_get (Variables|Default|GetSpringCoeff)))) (Transformation|GetWorldLocation) "None")
  ;[1 1 1] Reduce the "wobbling" of the vehicle
  (Class|PrimitiveComponent|SetAngularDamping _carmesh (Variables|Default|GetAngularDamping))
  (Variables|Default|SetPrevHit (Variables|Default|GetDistanceHit)))
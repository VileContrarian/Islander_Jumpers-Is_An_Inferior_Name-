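; Base hover vehicle: a physics-simulated car body held up by four thruster components, with input handled by BP_VehicleController.
; BeginPlay configures the thrusters, center of mass and health UI.
; Tick derives grounded state from two thrusters, scales engine volume with speed and checks health.
; Death spawns explosion effects and a wreck, hides the car, then a timer respawns and heals it using checkpoint actors; tilt-compensation logic exists but is unwired.
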(event Custom|Car_Speed_Sounds
  ;[1 1 1] Change Car Sounds based on Speed
  (Audio|Components|Audio|SetVolumeMultiplier (Variables|Default|GetCarAudioHigh) (Math|Float|Lerp 0.005 (Variables|Default|GetVolumeMax) (/ (Class|VehicleBase|GetSpeed) (Variables|Default|GetspeedMax))) :!class /Script/Engine.AudioComponent))

(event EventBeginPlay
  (CallFunction|InitThrusters)
  (Class|PrimitiveComponent|SetCenterOfMass (Variables|Default|GetCarBody) (Variables|Default|GetCenterOfMass) "None")
  (Variables|Default|SetInitialMaxSpeed (Variables|Default|GetspeedMax))
  (bind _returnvalue (UserInterface|CreateWidget "/Game/GameContent/Blueprints/UI/UIHealth.UIHealth_C"))
  (UserInterface|Viewport|AddtoViewport _returnvalue 0))

(event EventTick
  (params (DeltaSeconds :type Float%20%28single-precision%29))
  (CallFunction|GroundCheck)
  (CallFunction|CheckHealth)
  (CallFunction|CarSpeedSounds))

(event Input|ActionEvents|InputActionJump
  (params (Key :type Key%20Structure))
  ;[1 1 1 1 12] Control is being taken care of by BP_VehicleController. This input implementation will just be used for debugging or testing.
)

(event Input|ActionEvents|InputActionHandBrake
  (params (Key :type Key%20Structure))
  ;[1 1 1 1 12] Control is being taken care of by BP_VehicleController. This input implementation will just be used for debugging or testing.
)

(event Input|AxisEvents|InputAxisMoveForward
  (params (AxisValue :type Float%20%28single-precision%29))
  ;[1 1 1 1 12] Control is being taken care of by BP_VehicleController. This input implementation will just be used for debugging or testing.
)

(event Input|AxisEvents|InputAxisMoveSide
  (params (AxisValue :type Float%20%28single-precision%29))
  ;[1 1 1 1 12] Control is being taken care of by BP_VehicleController. This input implementation will just be used for debugging or testing.
)

(fn ConstructionScript
  (bind _carbody (Variables|Default|GetCarBody))
  (Class|VehicleBase|GetCarMesh _carbody)
  (Physics|SetSimulatePhysics _carbody true)
  (Class|PrimitiveComponent|SetMassOverrideinKg _carbody "None" (Variables|Default|Getmass) true))

(fn InitThrusters
  (bind _thruster2 (Variables|Default|GetThruster2))
  (bind _thruster1 (Variables|Default|GetThruster1))
  (bind _thruster3 (Variables|Default|GetThruster3))
  (bind _thruster4 (Variables|Default|GetThruster4))
  (Default|InitComponent _thruster1 (Variables|Default|GetCarBody))
  (Variables|/Game/GameContent/Blueprints/VehicleBase/BP_HoverComponent.BP_HoverComponent_C|SetHoverForce _thruster1 (Variables|Default|GetHoverForce))
  (Variables|/Game/GameContent/Blueprints/VehicleBase/BP_HoverComponent.BP_HoverComponent_C|SetHoverForce _thruster2 (Variables|Default|GetHoverForce))
  (Variables|/Game/GameContent/Blueprints/VehicleBase/BP_HoverComponent.BP_HoverComponent_C|SetHoverForce _thruster3 (Variables|Default|GetHoverForce))
  (Variables|/Game/GameContent/Blueprints/VehicleBase/BP_HoverComponent.BP_HoverComponent_C|SetHoverForce _thruster4 (Variables|Default|GetHoverForce))
  (Variables|/Game/GameContent/Blueprints/VehicleBase/BP_HoverComponent.BP_HoverComponent_C|SetTraceLength _thruster1 (Variables|Default|GetTraceLength))
  (Variables|/Game/GameContent/Blueprints/VehicleBase/BP_HoverComponent.BP_HoverComponent_C|SetTraceLength _thruster2 (Variables|Default|GetTraceLength))
  (Variables|/Game/GameContent/Blueprints/VehicleBase/BP_HoverComponent.BP_HoverComponent_C|SetTraceLength _thruster3 (Variables|Default|GetTraceLength))
  (Variables|/Game/GameContent/Blueprints/VehicleBase/BP_HoverComponent.BP_HoverComponent_C|SetTraceLength _thruster4 (Variables|Default|GetTraceLength))
  (Variables|/Game/GameContent/Blueprints/VehicleBase/BP_HoverComponent.BP_HoverComponent_C|SetAngularDamping _thruster1 (Variables|Default|GetAngularDamping))
  (Variables|/Game/GameContent/Blueprints/VehicleBase/BP_HoverComponent.BP_HoverComponent_C|SetAngularDamping _thruster2 (Variables|Default|GetAngularDamping))
  (Variables|/Game/GameContent/Blueprints/VehicleBase/BP_HoverComponent.BP_HoverComponent_C|SetAngularDamping _thruster3 (Variables|Default|GetAngularDamping))
  (Variables|/Game/GameContent/Blueprints/VehicleBase/BP_HoverComponent.BP_HoverComponent_C|SetAngularDamping _thruster4 (Variables|Default|GetAngularDamping)))

(fn GroundCheck
  (if (and (Variables|/Game/GameContent/Blueprints/VehicleBase/BP_HoverComponent.BP_HoverComponent_C|GetisHitGround (Variables|Default|GetThruster2)) (Variables|/Game/GameContent/Blueprints/VehicleBase/BP_HoverComponent.BP_HoverComponent_C|GetisHitGround (Variables|Default|GetThruster1)))
    (Variables|Default|SetisGrounded true)
    (else
      (Variables|Default|SetisGrounded false))))

(fn CheckHealth
  (if (not (Variables|Default|GetIsDead))
    (if (<= (Class|VehicleBase|GetHealth) 0)
      (CallFunction|OnDeath))))

(fn RotationalOrientationTracker
  (bind _carbody (Variables|Default|GetCarBody))
  (bind _returnvalue (Transformation|GetWorldRotation _carbody))
  (if (Variables|Default|GetisGrounded)
    (if (or (> (.pitch _returnvalue) 5.0) (< (.pitch _returnvalue) -5.0))
      (Variables|Default|SetTiltAngle (.pitch _returnvalue))
      (else
        (Variables|Default|SetTiltAngle 0.0)))
    (if (== (Variables|Default|GetTiltAngle) 0.0)
      (Variables|/Game/GameContent/Blueprints/VehicleBase/BP_HoverComponent.BP_HoverComponent_C|SetHoverForce (Variables|Default|GetThruster1) (Variables|Default|GetHoverForce))
      (Variables|/Game/GameContent/Blueprints/VehicleBase/BP_HoverComponent.BP_HoverComponent_C|SetHoverForce (Variables|Default|GetThruster2) (Variables|Default|GetHoverForce))
      (Variables|/Game/GameContent/Blueprints/VehicleBase/BP_HoverComponent.BP_HoverComponent_C|SetHoverForce (Variables|Default|GetThruster4) (Variables|Default|GetHoverForce))
      (Variables|/Game/GameContent/Blueprints/VehicleBase/BP_HoverComponent.BP_HoverComponent_C|SetHoverForce (Variables|Default|GetThruster3) (Variables|Default|GetHoverForce))
      (elif (> (Variables|Default|GetTiltAngle) 5.0)
        (Variables|/Game/GameContent/Blueprints/VehicleBase/BP_HoverComponent.BP_HoverComponent_C|SetHoverForce (Variables|Default|GetThruster1) 8e+01)
        (Variables|/Game/GameContent/Blueprints/VehicleBase/BP_HoverComponent.BP_HoverComponent_C|SetHoverForce (Variables|Default|GetThruster2) 8e+01)
        (elif (< (Variables|Default|GetTiltAngle) -5.0)
          (Variables|/Game/GameContent/Blueprints/VehicleBase/BP_HoverComponent.BP_HoverComponent_C|SetHoverForce (Variables|Default|GetThruster4) 6e+01)
          (Variables|/Game/GameContent/Blueprints/VehicleBase/BP_HoverComponent.BP_HoverComponent_C|SetHoverForce (Variables|Default|GetThruster3) 6e+01))))))

(fn TimedLoop
  (params (DeltaTime :type Float%20%28single-precision%29)))

(fn RespawnVehicle
  (bind _outactors (Actor|GetAllActorsOfClass "/Game/GameContent/Blueprints/BP_Checkpoint.BP_Checkpoint_C"))
  (for _array_element _outactors
    (Class|VehicleBase|Respawn _array_element)
    (Collision|SetCollisionEnabled (Variables|Default|GetCarBody) "QueryAndPhysics")
    (Variables|Default|SetIsDead false)
    (Input|EnableInput 0)
    (Class|VehicleBase|DoHeal (Class|VehicleBase|GetMaxHealth))
    (Rendering|SetVisibility (Variables|Default|GetCarShape) true false)
    (Physics|SetEnableGravity (Variables|Default|GetCarBody) true)))

(fn OnDeath
  (bind _carbody (Variables|Default|GetCarBody))
  (bind _carbody_2 (Variables|Default|GetCarBody))
  (bind _returnvalue (Transformation|GetWorldLocation _carbody))
  ;[1 1 1] On Death
  (Variables|Default|SetIsDead true)
  (Input|DisableInput 0)
  (Effects|SpawnEmitteratLocation "/Game/StarterContent/Particles/P_Explosion.P_Explosion" _returnvalue)
  (Effects|SpawnEmitteratLocation "/Game/StarterContent/Particles/P_Fire.P_Fire" _returnvalue)
  (Physics|SetPhysicsLinearVelocity _carbody_2 "0, 0, 0" false "None")
  (Class|PrimitiveComponent|SetPhysicsAngularVelocityinDegrees _carbody_2 "0, 0, 0" false "None")
  (Physics|SetEnableGravity _carbody_2 false)
  (Audio|PlaySoundatLocation "/Game/Audio/Death_Sound.Death_Sound" "0, 0, 0" "0, 0, 0" 1.0 1.0 0.0 0 0 0)
  (Collision|SetCollisionEnabled (Variables|Default|GetCarBody) "PhysicsOnly")
  (Rendering|SetVisibility (Variables|Default|GetCarShape) false false)
  (Game|SpawnActorfromClass "/Game/GameContent/Blueprints/BP_VehicleDestroyed.BP_VehicleDestroyed_C" (Transformation|GetWorldTransform (Variables|Default|GetCarBody)) "Undefined" 0 0)
  ;;[1 1 1 1 12] Call the respawn after set time has passed (Revive Cooldown)
  (Utilities|Time|SetTimerbyFunctionName 0 "RespawnVehicle" 2.0))
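; Hover car component that pushes a car mesh, supplied through InitComponent, away from the surface beneath it.
; Each tick it traces along its down vector and, on a hit, applies force at its own location along the impact normal, fading linearly with distance, and sets the mesh's damping.
; Without a hit, it flags itself airborne and adds a gravity velocity to the mesh.
; An alternative spring-damper method is present but disconnected.
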(event Custom|InitComponent
  (params (Mesh%20Component :type Static%20Mesh%20Component%20Object%20Reference))
  (Variables|Default|SetCarMesh Mesh%20Component))

(event EventBeginPlay)

(event EventTick
  (params (DeltaSeconds :type Float%20%28single-precision%29))
  (bind _returnvalue (Transformation|GetWorldLocation))
  (bind _carmesh (Variables|Default|GetCarMesh))
  ;[1 1 1] Raycast
  (bind _outhit (Collision|LineTraceByChannel _returnvalue (+ _returnvalue (* (Math|Vector|GetUpVector) (* (Variables|Default|GetTraceLength) -1.0))) "TraceTypeQuery1" false 0 "ForOneFrame"))
  (if (.bBlockingHit (Collision|BreakHitResult _outhit))
    (Variables|Default|SetisOnTheGround true)
    ;[1 1 1] Method 1
    (Class|PrimitiveComponent|AddForceatLocation _carmesh (* (.ImpactNormal (Collision|BreakHitResult _outhit)) (Math|Float|Lerp (* (Variables|Default|GetHoverForce) 1e+04) 0.0 (/ (Math|Vector|VectorLength (- (Transformation|GetWorldLocation) (.Location (Collision|BreakHitResult _outhit)))) (Variables|Default|GetTraceLength)))) (Transformation|GetWorldLocation) "None")
    (Class|PrimitiveComponent|SetLinearDamping _carmesh (Variables|Default|GetLinearDamping))
    (Class|PrimitiveComponent|SetAngularDamping _carmesh (Variables|Default|GetAngularDamping))
    (else
      (Variables|Default|SetisOnTheGround false)
      ;[1 1 1] Gravity
      (Development|PrintString "")
      (Physics|SetPhysicsLinearVelocity (Variables|Default|GetCarMesh) (Math|Vector|MakeVector 0.0 0.0 (Variables|Default|GetgravityForce)) true "None"))))
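; Player-driven hovercar physics Blueprint, held up by four hover components that share one hover force and trace length set on BeginPlay.
; The construction script binds each component to CarMesh, and GroundCheck treats the car as grounded only when both front components report ground.
; When grounded, throttle applies force along the horizontal forward vector and jump adds velocity along mesh up.
; Steering directly sets yaw angular velocity, even when airborne.
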(event EventBeginPlay
  (CallFunction|SetAllHoverForce)
  (CallFunction|SetAllTraceLength))

(event Collision|EventActorBeginOverlap
  (params (OtherActor :type Actor%20Object%20Reference)))

(event EventTick
  (params (DeltaSeconds :type Float%20%28single-precision%29)))

(event Input|ActionEvents|InputActionJump
  (params (Key :type Key%20Structure))
  (bind _carmesh (Variables|Default|GetCarMesh))
  (:Pressed
    (CallFunction|GroundCheck)
    (if (Variables|Default|GetisGrounded)
      (Physics|SetPhysicsLinearVelocity _carmesh (* (Math|Vector|GetUpVector _carmesh) (Variables|Default|GetJumpForce)) true "None"))))

(event Input|AxisEvents|InputAxisMoveForward
  (params (AxisValue :type Float%20%28single-precision%29))
  (bind _carmesh (Variables|Default|GetCarMesh))
  (bind _returnvalue (Math|Vector|GetForwardVector _carmesh))
  (CallFunction|GroundCheck)
  (if (Variables|Default|GetisGrounded)
    (Physics|AddForce (Variables|Default|GetCarMesh) (* (* (Math|Vector|MakeVector (.x _returnvalue) (.y _returnvalue) 0.0) 1e+07) AxisValue) "None" false)))

(event Input|AxisEvents|InputAxisMoveSide
  (params (AxisValue :type Float%20%28single-precision%29))
  (Class|PrimitiveComponent|SetPhysicsAngularVelocityinRadians (Variables|Default|GetCarMesh) (Math|Vector|MakeVector 0.0 0.0 (* AxisValue 1e+01)) false "None"))

(fn ConstructionScript
  (bind _carmesh (Variables|Default|GetCarMesh))
  (Default|InitComponent (Variables|Default|GetHoverComponent1) _carmesh)
  (Default|InitComponent (Variables|Default|GetHoverComponent2) _carmesh)
  (Default|InitComponent (Variables|Default|GetHoverComponent3) _carmesh)
  (Default|InitComponent (Variables|Default|GetHoverComponent4) _carmesh))

(fn SetAllHoverForce
  (bind _allhoverforce (Variables|Default|GetAllHoverForce))
  (Variables|/Game/GameContent/Blueprints/HoverCar/HoverComponent.HoverComponent_C|SetHoverForce (Variables|Default|GetHoverComponent1) _allhoverforce)
  (Variables|/Game/GameContent/Blueprints/HoverCar/HoverComponent.HoverComponent_C|SetHoverForce (Variables|Default|GetHoverComponent2) _allhoverforce)
  (Variables|/Game/GameContent/Blueprints/HoverCar/HoverComponent.HoverComponent_C|SetHoverForce (Variables|Default|GetHoverComponent3) _allhoverforce)
  (Variables|/Game/GameContent/Blueprints/HoverCar/HoverComponent.HoverComponent_C|SetHoverForce (Variables|Default|GetHoverComponent4) _allhoverforce))

(fn SetAllLinearDamping)

(fn SetAllAngularDamping)

(fn SetAllTraceLength
  (bind _alltracelength (Variables|Default|GetAllTraceLength))
  (Variables|/Game/GameContent/Blueprints/HoverCar/HoverComponent.HoverComponent_C|SetTraceLength (Variables|Default|GetHoverComponent1) _alltracelength)
  (Variables|/Game/GameContent/Blueprints/HoverCar/HoverComponent.HoverComponent_C|SetTraceLength (Variables|Default|GetHoverComponent2) _alltracelength)
  (Variables|/Game/GameContent/Blueprints/HoverCar/HoverComponent.HoverComponent_C|SetTraceLength (Variables|Default|GetHoverComponent3) _alltracelength)
  (Variables|/Game/GameContent/Blueprints/HoverCar/HoverComponent.HoverComponent_C|SetTraceLength (Variables|Default|GetHoverComponent4) _alltracelength))

(fn GroundCheck
  ;[1 1 1] IF Front Wheels are on the ground
  (if (and (Variables|/Game/GameContent/Blueprints/HoverCar/HoverComponent.HoverComponent_C|GetisOnTheGround (Variables|Default|GetHoverComponent1)) (Variables|/Game/GameContent/Blueprints/HoverCar/HoverComponent.HoverComponent_C|GetisOnTheGround (Variables|Default|GetHoverComponent2)))
    (Variables|Default|SetisGrounded true)
    (else
      (Variables|Default|SetisGrounded false))))
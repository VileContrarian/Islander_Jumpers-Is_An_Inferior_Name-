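; Test game mode that sets up local players, each with a vehicle, when play begins.
; BeginPlay caches all PlayerStart actors, then loops over player indices up to NumberOfPlayers to find starts whose PlayerStartTag equals the index as a name.
; For each match it creates the player, spawns a BP_VehicleBase01 at that start's transform and has that player's controller possess it.
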(event EventBeginPlay
  ;[1 1 1] Gives Player A Controller When Joining Game
  (CallFunction|GetAllActors)
  (CallFunction|Spawn))

(event EventTick
  (params (DeltaSeconds :type Float%20%28single-precision%29)))

(fn ConstructionScript)

(fn Spawn
  (for _index (range 0 (Variables|Default|GetNumberOfPlayers))
    (Variables|Default|SetPlayerIndex _index)
    (for _array_element (Variables|Default|GetPlayers)
      ;[1 1 1] Creates a Player and Spawns Vehicle
      (if (Utilities|Name|Equal(Name) (Variables|/Script/Engine.PlayerStart|GetPlayerStartTag _array_element) (Utilities|String|StringToName (Utilities|String|ToString(Integer) (Variables|Default|GetPlayerIndex))))
        (Class|GameplayStatics|CreatePlayer (Variables|Default|GetPlayerIndex))
        (bind _returnvalue (Game|SpawnActorfromClass "/Game/GameContent/Blueprints/BP_VehicleBase01.BP_VehicleBase01_C" (Transformation|GetActorTransform _array_element) "Undefined" 0 0))
        (Pawn|Possess (Game|GetPlayerController (Variables|Default|GetPlayerIndex)) _returnvalue)))))

(fn GetAllActors
  (bind _outactors (Actor|GetAllActorsOfClass "/Script/Engine.PlayerStart"))
  (Variables|Default|SetPlayers _outactors))
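; Player controller that relays player input to a vehicle in the level.
; On BeginPlay it takes the first actor implementing I_ControlsInput and caches it as a BP_VehicleBase01 reference, without possessing it.
; Movement axes, Jump and HandBrake press/release are forwarded to that vehicle as event messages, each guarded by a validity check.
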(event EventBeginPlay
  (bind _outactors (Actor|GetAllActorswithInterface "/Game/GameContent/Blueprints/I_ControlsInput.I_ControlsInput_C"))
  (if (Utilities|Array|IsValidIndex _outactors)
    (bind _asbp_vehicle_base_01 (Utilities|Casting|CastToBP_VehicleBase01 (Utilities|Array|Get(acopy) _outactors)))
    (Variables|Default|SetVehicleObject _asbp_vehicle_base_01)))

(event EventTick
  (params (DeltaSeconds :type Float%20%28single-precision%29)))

(event Input|ActionEvents|InputActionJump
  (params (Key :type Key%20Structure))
  (bind _vehicleobject (Variables|Default|GetVehicleObject))
  (:Pressed
    (Utilities|IsValid _vehicleobject
      (:Is%20Valid
        (Class|IControlsInput|JumpEvent(Message) _vehicleobject)))))

(event Input|ActionEvents|InputActionHandBrake
  (params (Key :type Key%20Structure))
  (bind _vehicleobject (Variables|Default|GetVehicleObject))
  (:Pressed
    (Utilities|IsValid _vehicleobject
      (:Is%20Valid
        (Class|IControlsInput|HandBrakeonEvent(Message) _vehicleobject))))
  (:Released
    (Utilities|IsValid _vehicleobject
      (:Is%20Valid
        (Class|IControlsInput|HandBrakeOffEvent(Message) _vehicleobject)))))

(event Input|AxisEvents|InputAxisMoveForward
  (params (AxisValue :type Float%20%28single-precision%29))
  (bind _vehicleobject (Variables|Default|GetVehicleObject))
  (Utilities|IsValid _vehicleobject
    (:Is%20Valid
      (Class|IControlsInput|MoveForwardEvent(Message) _vehicleobject AxisValue))))

(event Input|AxisEvents|InputAxisMoveSide
  (params (AxisValue :type Float%20%28single-precision%29))
  (bind _vehicleobject (Variables|Default|GetVehicleObject))
  (Utilities|IsValid _vehicleobject
    (:Is%20Valid
      (Class|IControlsInput|MoveRightEvent(Message) _vehicleobject AxisValue))))

(fn ConstructionScript)
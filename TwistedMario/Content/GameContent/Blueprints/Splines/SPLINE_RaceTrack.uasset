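; Race track spline actor that populates its TrackPath spline with randomly chosen point actors when play begins.
; BeginPlay counts the spline points, then loops from index 2 up to that count, calling BuildElement for each.
; BuildElement stores the index and calls ChooseElement, which spawns either SA_Point or PillarSA_Point at random, using that point's world transform without scale.
; A wrapped next-point index is computed but not used here.
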(event EventBeginPlay
  (Utilities|FlowControl|Sequence
    (:then_0
      (Variables|Default|SetSplinePoints (Spline|GetNumberOfSplinePoints (Variables|Default|GetTrackPath))))
    (:then_1
      (for _index (range 2 (Variables|Default|GetSplinePoints))
        (CallFunction|BuildElement _index)))))

(event Collision|EventActorBeginOverlap
  (params (OtherActor :type Actor%20Object%20Reference)))

(event EventTick
  (params (DeltaSeconds :type Float%20%28single-precision%29)))

(fn ConstructionScript)

(fn BuildElement
  (params (LoopIndex :type Integer))
  (Variables|Default|SetCurrentLoopIndex LoopIndex)
  (Variables|Default|SetNextLoopIndex (Math|Integer|%(Integer) (+ LoopIndex 1) (Variables|Default|GetSplinePoints)))
  (if (not (> (Variables|Default|GetCurrentLoopIndex) (Variables|Default|GetSplinePoints)))
    (CallFunction|ChooseElement)))

(fn ChooseElement
  (switch int (Math|Random|RandomIntegerinRange 0 1)
    (:0
      (Game|SpawnActorfromClass "/Game/GameContent/Blueprints/Blockers/SA_Point.SA_Point_C" (Spline|GetTransformatSplinePoint (Variables|Default|GetTrackPath) (Variables|Default|GetCurrentLoopIndex) "World" false) "Undefined" 0 0))
    (:1
      (Game|SpawnActorfromClass "/Game/GameContent/Blueprints/Blockers/PillarSA_Point.PillarSA_Point_C" (Spline|GetTransformatSplinePoint (Variables|Default|GetTrackPath) (Variables|Default|GetCurrentLoopIndex) "World" false) "Undefined" 0 0))))
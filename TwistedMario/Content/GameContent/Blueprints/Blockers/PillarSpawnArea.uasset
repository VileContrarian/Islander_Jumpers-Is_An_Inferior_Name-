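; PillarSpawnArea is a blocker area that has an even chance of containing one pillar at a randomly chosen spot.
; Its construction script caches the relative transforms of five marker components as spawn points, then rolls whether to spawn.
; On success, SpawnPillar adds a child actor component at a random one of those transforms.
; All placement happens at construction, with the event graph left unused.
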(event EventBeginPlay)

(event Collision|EventActorBeginOverlap
  (params (OtherActor :type Actor%20Object%20Reference)))

(event EventTick
  (params (DeltaSeconds :type Float%20%28single-precision%29)))

(fn ConstructionScript
  (CallFunction|SetSpawnPoints)
  (switch int (Math|Random|RandomIntegerinRange 0 1)
    (:0
      (CallFunction|SpawnPillar))))

(fn SetSpawnPoints
  (Variables|Default|SetSpawn_Points (Utilities|Array|MakeArray (Transformation|GetRelativeTransform (Variables|Default|GetSPN_1_R)) (Transformation|GetRelativeTransform (Variables|Default|GetSPN_2_L)) (Transformation|GetRelativeTransform (Variables|Default|GetSPN_3_SIDEWAYS)) (Transformation|GetRelativeTransform (Variables|Default|GetSPN_4_DIAGONAL)) (Transformation|GetRelativeTransform (Variables|Default|GetSPN_5_MID)))))

(fn SpawnPillar
  (bind _spawn_points (Variables|Default|GetSpawn_Points))
  (AddComponent|AddChildActorComponent false (Utilities|Array|Get(acopy) _spawn_points (Math|Random|RandomIntegerinRange 0 (Utilities|Array|LastIndex _spawn_points)))))
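; Blocker spawn area actor that randomly fills itself with snowpile and rock obstacles.
; The construction script caches five marker transforms (right, left, up, down, middle), then rolls for snowpiles, a rock, both, or nothing, with snowpiles weighted higher.
; Each blocker is a child actor component placed at a randomly picked marker, so picks can overlap.
; The event graph is unused; all spawning happens at construction.
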(event EventBeginPlay)

(event Collision|EventActorBeginOverlap
  (params (OtherActor :type Actor%20Object%20Reference)))

(event EventTick
  (params (DeltaSeconds :type Float%20%28single-precision%29)))

(fn ConstructionScript
  (CallFunction|SetSpawnPoints)
  (switch int (Math|Random|RandomIntegerinRange 0 4)
    (:0
      (CallFunction|SpawnSnowpiles))
    (:1
      (CallFunction|SpawnRocks))
    (:2
      (CallFunction|SpawnSnowpiles))
    (:3
      (CallFunction|SpawnSnowandRock))))

(fn SetSpawnPoints
  (Variables|Default|SetSpawn_Points (Utilities|Array|MakeArray (Transformation|GetRelativeTransform (Variables|Default|GetSPN_1_R)) (Transformation|GetRelativeTransform (Variables|Default|GetSPN_2_L)) (Transformation|GetRelativeTransform (Variables|Default|GetSPN_3_UP)) (Transformation|GetRelativeTransform (Variables|Default|GetSPN_4_DOWN)) (Transformation|GetRelativeTransform (Variables|Default|GetSPN_5_MID)))))

(fn SpawnSnowpiles
  (bind _spawn_points (Variables|Default|GetSpawn_Points))
  (for _index (range 0 (Math|Random|RandomIntegerinRange 0 3))
    (AddComponent|AddChildActorComponent false (Utilities|Array|Get(acopy) _spawn_points (Math|Random|RandomIntegerinRange 0 (Utilities|Array|LastIndex _spawn_points))))))

(fn SpawnRocks
  (bind _spawn_points (Variables|Default|GetSpawn_Points))
  (AddComponent|AddChildActorComponent false (Utilities|Array|Get(acopy) _spawn_points (Math|Random|RandomIntegerinRange 0 (Utilities|Array|LastIndex _spawn_points)))))

(fn SpawnSnowandRock
  (CallFunction|SpawnSnowpiles)
  (CallFunction|SpawnRocks))
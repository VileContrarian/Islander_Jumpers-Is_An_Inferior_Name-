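; Spline path actor that places BP_ItemSpawn item spawners along its curve when play begins.
; Spawner steps along the spline at Spacing intervals from the fourth one onward, so larger spacing yields fewer spawners.
; Each spawner sits slightly below the spline and takes only the yaw toward the next sample point to follow the curve.
; The construction script loops over spline points but does nothing.
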(event EventBeginPlay
  (CallFunction|Spawner))

(event Collision|EventActorBeginOverlap
  (params (OtherActor :type Actor%20Object%20Reference)))

(event EventTick
  (params (DeltaSeconds :type Float%20%28single-precision%29)))

(fn ConstructionScript
  (for _index (range 0 (- (Spline|GetNumberOfSplinePoints (Variables|Default|GetSpline)) 2))
    _))

(fn Spawner
  (params (ObjectToSpawn :type Actor%20Object%20Reference))
  (bind _spline (Variables|Default|GetSpline))
  (bind _spacing (Variables|Default|GetSpacing))
  (for _index (range 3 (- (.ReturnValue (Math|Float|Division(WholeandRemainder) (Spline|GetSplineLength (Variables|Default|GetSpline)) _spacing)) 1))
    (Game|SpawnActorfromClass "/Game/GameContent/Blueprints/ItemGeneration/BP_ItemSpawn.BP_ItemSpawn_C" (Math|Transform|MakeTransform (Math|Vector|MakeVector (.x (Spline|GetLocationatDistanceAlongSpline _spline (* _index _spacing) "World")) (.y (Spline|GetLocationatDistanceAlongSpline _spline (* _index _spacing) "World")) (- (.z (Spline|GetLocationatDistanceAlongSpline _spline (* _index _spacing) "World")) 5e+01)) (Math|Rotator|MakeRotator 0.0 0.0 (.yaw (Math|Rotator|FindLookatRotation (Math|Vector|MakeVector (.x (Spline|GetLocationatDistanceAlongSpline _spline (* _index _spacing) "World")) (.y (Spline|GetLocationatDistanceAlongSpline _spline (* _index _spacing) "World")) (.z (Spline|GetLocationatDistanceAlongSpline _spline (* _index _spacing) "World"))) (Spline|GetLocationatDistanceAlongSpline _spline (* (+ _index 1) _spacing) "World"))))) "Undefined" 0 0)))
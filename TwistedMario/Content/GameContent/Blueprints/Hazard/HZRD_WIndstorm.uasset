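; Windstorm hazard actor that travels along a track spline and punishes the player's vehicle while it is inside.
; If active, a timeline moves it along TrackRef's StormPath spline, with configurable duration and start offset.
; InnerCollision overlaps toggle InStorm, and StormDamage runs every Tick, damaging player pawn 0 and lowering its max speed to a floor.
; Four seconds after a vehicle exits, that vehicle's max speed resets to a fixed value.
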(event OnComponentBeginOverlap(InnerCollision)
  (params (OverlappedComponent :type Primitive%20Component%20Object%20Reference) (OtherActor :type Actor%20Object%20Reference) (OtherComp :type Primitive%20Component%20Object%20Reference) (OtherBodyIndex :type Integer) (bFromSweep :type Boolean) (SweepResult :type Hit%20Result%20Structure%20%28by%20ref%29))
  (bind _asvehicle_base (Utilities|Casting|CastToVehicleBase OtherActor))
  (Utilities|Casting|CastToBP_VehicleBase01 _asvehicle_base)
  (Variables|Default|SetInStorm true)
  (CallFunction|StormDamage))

(event OnComponentEndOverlap(InnerCollision)
  (params (OverlappedComponent :type Primitive%20Component%20Object%20Reference) (OtherActor :type Actor%20Object%20Reference) (OtherComp :type Primitive%20Component%20Object%20Reference) (OtherBodyIndex :type Integer))
  (bind _asvehicle_base (Utilities|Casting|CastToVehicleBase OtherActor))
  (bind _asbp_vehicle_base_01 (Utilities|Casting|CastToBP_VehicleBase01 _asvehicle_base))
  (Variables|Default|SetInStorm false)
  (CallFunction|StormDamage)
  (Utilities|FlowControl|Delay 4.0)
  (Variables|/Script/TwistedMario.VehicleBase|SetspeedMax _asbp_vehicle_base_01 3e+02))

(event Custom|MoveStorm
  (Components|Timeline|SetPlayRate (Variables|Default|GetStormPath) (/ 1.0 (Variables|Default|GetDuration)))
  (Components|Timeline|SetNewTime (Variables|Default|GetStormPath) (Variables|Default|GetStartOffset))
  (bind _alpha (Timeline|StormPath Play)
    (:Update
      (Variables|Default|SetAlpha _alpha)
      (Transformation|SetActorLocationAndRotation (Spline|GetLocationatDistanceAlongSpline (Variables|/Game/GameContent/Blueprints/Splines/SPLINE_Storm.SPLINE_Storm_C|GetStormPath (Variables|Default|GetTrackRef)) (Math|Float|Lerp 0.0 (Spline|GetSplineLength (Variables|/Game/GameContent/Blueprints/Splines/SPLINE_Storm.SPLINE_Storm_C|GetStormPath (Variables|Default|GetTrackRef))) (Variables|Default|GetAlpha)) "World") (Transformation|GetActorRotation)))))

(event EventBeginPlay
  (if (Variables|Default|GetActiveStorm)
    (CallFunction|MoveStorm)))

(event Collision|EventActorBeginOverlap
  (params (OtherActor :type Actor%20Object%20Reference)))

(event EventTick
  (params (DeltaSeconds :type Float%20%28single-precision%29))
  (CallFunction|StormDamage))

(fn ConstructionScript)

(fn StormDamage
  (if (Variables|Default|GetInStorm)
    (bind _asbp_vehicle_base_01 (Utilities|Casting|CastToBP_VehicleBase01 (Game|Player|GetPlayerPawn 0)))
    (Class|VehicleBase|DoDamage _asbp_vehicle_base_01 10)
    ;[1 1 1] If Car's Max Speed is under 120: keep it there. Otherwise Lower It while it's in the Storm
    (if (< (Variables|/Script/TwistedMario.VehicleBase|GetspeedMax _asbp_vehicle_base_01) 1e+02)
      ;[1 1 1] Remove Max Speed, unless it's at 120
      (Variables|/Script/TwistedMario.VehicleBase|SetspeedMax _asbp_vehicle_base_01 1e+02)
      (else
        (Variables|/Script/TwistedMario.VehicleBase|SetspeedMax _asbp_vehicle_base_01 (- (Variables|/Script/TwistedMario.VehicleBase|GetspeedMax _asbp_vehicle_base_01) 1e+01))))))
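; Base hover vehicle pawn: a physics-simulated car body held up by four thruster components.
; Construction sets up the body and mass; BeginPlay applies the center of mass and passes shared hover force, trace length and damping to the thrusters.
; Each tick it counts as grounded when thrusters 1 and 2 both hit ground.
; It also checks health every tick, asking BP_MainLocalGameMode to kill its controller at zero or below.
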(event EventBeginPlay
  (CallFunction|InitThrusters)
  (Class|PrimitiveComponent|SetCenterOfMass (Variables|Default|GetCarBody) (Variables|Default|GetCenterOfMass) "None"))

(event EventTick
  (params (DeltaSeconds :type Float%20%28single-precision%29))
  (CallFunction|GroundCheck)
  (Utilities|FlowControl|DoOnce false :!label _label
    (:Completed
      (CallFunction|CheckHealth)
      (goto _label Reset))))

(fn ConstructionScript
  (bind _carbody (Variables|Default|GetCarBody))
  (Class|VehicleBase|GetCarMesh _carbody)
  (Physics|SetSimulatePhysics _carbody true)
  (Class|PrimitiveComponent|SetMassOverrideinKg _carbody "None" (Variables|Default|Getmass) true))

(fn InitThrusters
  (bind _thurster1 (Variables|Default|GetThurster1))
  (bind _thruster2 (Variables|Default|GetThruster2))
  (bind _thruster3 (Variables|Default|GetThruster3))
  (bind _thruster4 (Variables|Default|GetThruster4))
  (Default|InitComponent _thruster2 (Variables|Default|GetCarBody))
  (Variables|/Game/GameContent/Blueprints/BP_HoverComponent.BP_HoverComponent_C|SetHoverForce _thurster1 (Variables|Default|GetHoverForce))
  (Variables|/Game/GameContent/Blueprints/BP_HoverComponent.BP_HoverComponent_C|SetHoverForce _thruster2 (Variables|Default|GetHoverForce))
  (Variables|/Game/GameContent/Blueprints/BP_HoverComponent.BP_HoverComponent_C|SetHoverForce _thruster3 (Variables|Default|GetHoverForce))
  (Variables|/Game/GameContent/Blueprints/BP_HoverComponent.BP_HoverComponent_C|SetHoverForce _thruster4 (Variables|Default|GetHoverForce))
  (Variables|/Game/GameContent/Blueprints/BP_HoverComponent.BP_HoverComponent_C|SetTraceLength _thurster1 (Variables|Default|GetTraceLength))
  (Variables|/Game/GameContent/Blueprints/BP_HoverComponent.BP_HoverComponent_C|SetTraceLength _thruster2 (Variables|Default|GetTraceLength))
  (Variables|/Game/GameContent/Blueprints/BP_HoverComponent.BP_HoverComponent_C|SetTraceLength _thruster3 (Variables|Default|GetTraceLength))
  (Variables|/Game/GameContent/Blueprints/BP_HoverComponent.BP_HoverComponent_C|SetTraceLength _thruster4 (Variables|Default|GetTraceLength))
  (Variables|/Game/GameContent/Blueprints/BP_HoverComponent.BP_HoverComponent_C|SetAngularDamping _thurster1 (Variables|Default|GetAngularDamping))
  (Variables|/Game/GameContent/Blueprints/BP_HoverComponent.BP_HoverComponent_C|SetAngularDamping _thruster2 (Variables|Default|GetAngularDamping))
  (Variables|/Game/GameContent/Blueprints/BP_HoverComponent.BP_HoverComponent_C|SetAngularDamping _thruster3 (Variables|Default|GetAngularDamping))
  (Variables|/Game/GameContent/Blueprints/BP_HoverComponent.BP_HoverComponent_C|SetAngularDamping _thruster4 (Variables|Default|GetAngularDamping)))

(fn GroundCheck
  (if (and (Variables|/Game/GameContent/Blueprints/BP_HoverComponent.BP_HoverComponent_C|GetisHitGround (Variables|Default|GetThruster2)) (Variables|/Game/GameContent/Blueprints/BP_HoverComponent.BP_HoverComponent_C|GetisHitGround (Variables|Default|GetThurster1)))
    (Variables|Default|SetisGrounded true)
    (else
      (Variables|Default|SetisGrounded false))))

(fn CheckHealth
  (if (<= (Class|VehicleBase|GetHealth) 0)
    (bind _asbp_main_local_game_mode (Utilities|Casting|CastToBP_MainLocalGameMode (Game|GetGameMode)))
    (bind _asbp_vehicle_controller (Utilities|Casting|CastToBP_VehicleController (Pawn|GetController)))
    (Default|Kill _asbp_main_local_game_mode _asbp_vehicle_controller)))
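; Base hover vehicle Blueprint: a physics-simulated car body suspended by four thruster components and driven by player input.
; Construction obtains the body mesh and overrides its mass; BeginPlay configures each thruster's hover force, trace length and damping, then sets center of mass.
; Tick sets IsGrounded only when Thruster1 and Thruster2 both hit ground.
; Inputs call Accelerate, Turn, Jump and handbrake functions defined outside these graphs; FallingState is unwired.
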(event EventBeginPlay
  (CallFunction|InitThrusters)
  (Class|PrimitiveComponent|SetCenterOfMass (Variables|Default|GetCarBody) (Variables|Default|GetCenterOfMass) "None"))

(event Collision|EventActorBeginOverlap
  (params (OtherActor :type Actor%20Object%20Reference)))

(event EventTick
  (params (DeltaSeconds :type Float%20%28single-precision%29))
  (CallFunction|GroundCheck))

(event Input|ActionEvents|InputActionJump
  (params (Key :type Key%20Structure))
  (:Pressed
    (Class|VehicleBase|Jump)))

(event Input|ActionEvents|InputActionHandBrake
  (params (Key :type Key%20Structure))
  (:Pressed
    (Class|VehicleBase|HandBrake))
  (:Released
    (Class|VehicleBase|ReleaseHandBrake)))

(event Input|AxisEvents|InputAxisMoveForward
  (params (AxisValue :type Float%20%28single-precision%29))
  (Class|VehicleBase|Accelerate AxisValue))

(event Input|AxisEvents|InputAxisMoveSide
  (params (AxisValue :type Float%20%28single-precision%29))
  (Class|VehicleBase|Turn AxisValue))

(fn ConstructionScript
  (bind _carbody (Variables|Default|GetCarBody))
  (Class|VehicleBase|GetCarMesh _carbody)
  (Physics|SetSimulatePhysics _carbody true)
  (Class|PrimitiveComponent|SetMassOverrideinKg _carbody "None" (Variables|Default|Getmass) true))

(fn InitThrusters
  (bind _thruster2 (Variables|Default|GetThruster2))
  (bind _thruster1 (Variables|Default|GetThruster1))
  (bind _thruster3 (Variables|Default|GetThruster3))
  (bind _thruster4 (Variables|Default|GetThruster4))
  (Default|InitComponent _thruster1 (Variables|Default|GetCarBody))
  (Variables|/Game/GameContent/BP_HoverComponent.BP_HoverComponent_C|SetHoverForce _thruster1 (Variables|Default|GetHoverForce))
  (Variables|/Game/GameContent/BP_HoverComponent.BP_HoverComponent_C|SetHoverForce _thruster2 (Variables|Default|GetHoverForce))
  (Variables|/Game/GameContent/BP_HoverComponent.BP_HoverComponent_C|SetHoverForce _thruster3 (Variables|Default|GetHoverForce))
  (Variables|/Game/GameContent/BP_HoverComponent.BP_HoverComponent_C|SetHoverForce _thruster4 (Variables|Default|GetHoverForce))
  (Variables|/Game/GameContent/BP_HoverComponent.BP_HoverComponent_C|SetTraceLength _thruster1 (Variables|Default|GetTraceLength))
  (Variables|/Game/GameContent/BP_HoverComponent.BP_HoverComponent_C|SetTraceLength _thruster2 (Variables|Default|GetTraceLength))
  (Variables|/Game/GameContent/BP_HoverComponent.BP_HoverComponent_C|SetTraceLength _thruster3 (Variables|Default|GetTraceLength))
  (Variables|/Game/GameContent/BP_HoverComponent.BP_HoverComponent_C|SetTraceLength _thruster4 (Variables|Default|GetTraceLength))
  (Variables|/Game/GameContent/BP_HoverComponent.BP_HoverComponent_C|SetAngularDamping _thruster1 (Variables|Default|GetAngularDamping))
  (Variables|/Game/GameContent/BP_HoverComponent.BP_HoverComponent_C|SetAngularDamping _thruster2 (Variables|Default|GetAngularDamping))
  (Variables|/Game/GameContent/BP_HoverComponent.BP_HoverComponent_C|SetAngularDamping _thruster3 (Variables|Default|GetAngularDamping))
  (Variables|/Game/GameContent/BP_HoverComponent.BP_HoverComponent_C|SetAngularDamping _thruster4 (Variables|Default|GetAngularDamping)))

(fn GroundCheck
  (if (and (Variables|/Game/GameContent/BP_HoverComponent.BP_HoverComponent_C|GetisHitGround (Variables|Default|GetThruster2)) (Variables|/Game/GameContent/BP_HoverComponent.BP_HoverComponent_C|GetisHitGround (Variables|Default|GetThruster1)))
    (Variables|Default|SetisGrounded true)
    (else
      (Variables|Default|SetisGrounded false))))
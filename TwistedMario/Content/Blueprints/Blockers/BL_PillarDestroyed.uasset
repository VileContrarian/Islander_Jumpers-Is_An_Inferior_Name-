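; BL_PillarDestroyed is a destructible pillar blocker that damages vehicles driving into it.
; When a BP_VehicleBase01 overlaps the collider, it takes damage and radius damage is applied to the destructible pillar at the car's location.
; When the pillar component fractures, it plays an OrbHit sound, then destroys the actor after a short delay.
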(event OnComponentFracture(D_Pillar)
  (params (HitPoint :type Vector%20%28by%20ref%29 :default "0, 0, 0") (HitDirection :type Vector%20%28by%20ref%29 :default "0, 0, 0"))
  (Audio|PlaySoundatLocation "/Game/Audio/orbHit.orbHit" (Transformation|GetActorLocation) "0, 0, 0" 1.0 1.0 0.0 0 0 0)
  (Utilities|FlowControl|Delay 3.0)
  (Actor|DestroyActor))

(event OnComponentBeginOverlap(Collider)
  (params (OverlappedComponent :type Primitive%20Component%20Object%20Reference) (OtherActor :type Actor%20Object%20Reference) (OtherComp :type Primitive%20Component%20Object%20Reference) (OtherBodyIndex :type Integer) (bFromSweep :type Boolean) (SweepResult :type Hit%20Result%20Structure%20%28by%20ref%29))
  (bind _asvehicle_base (Utilities|Casting|CastToVehicleBase OtherActor))
  (bind _asbp_vehicle_base_01 (Utilities|Casting|CastToBP_VehicleBase01 _asvehicle_base))
  (Class|VehicleBase|DoDamage _asbp_vehicle_base_01 12)
  (Class|DestructibleComponent|ApplyRadiusDamage (Variables|Default|GetD_Pillar) 5.0 (Transformation|GetWorldLocation (Variables|/Game/Blueprints/VehicleBase/BP_VehicleBase01.BP_VehicleBase01_C|GetCarShape _asbp_vehicle_base_01)) 0.0 0.0 false))

(event EventBeginPlay)

(event Collision|EventActorBeginOverlap
  (params (OtherActor :type Actor%20Object%20Reference)))

(event EventTick
  (params (DeltaSeconds :type Float%20%28single-precision%29)))

(fn ConstructionScript)
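; BL_Oil is an oil hazard that makes a vehicle temporarily slippery: slightly faster but much worse at turning.
; On collider overlap with a BP_VehicleBase01, it spawns an oil explosion and sound, then scales the vehicle's max speed and turn coefficient.
; Max speed is capped, and the turn coefficient floor applies only when that cap triggers.
; After a delay, both values reset to the vehicle's stored originals.
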(event OnComponentBeginOverlap(Collider)
  (params (OverlappedComponent :type Primitive%20Component%20Object%20Reference) (OtherActor :type Actor%20Object%20Reference) (OtherComp :type Primitive%20Component%20Object%20Reference) (OtherBodyIndex :type Integer) (bFromSweep :type Boolean) (SweepResult :type Hit%20Result%20Structure%20%28by%20ref%29))
  (bind _returnvalue (Transformation|GetActorLocation))
  (Utilities|IsValid OtherActor
    (:Is%20Valid
      (bind _asbp_vehicle_base_01 (Utilities|Casting|CastToBP_VehicleBase01 OtherActor))
      (Variables|Default|SetVehicleRef _asbp_vehicle_base_01)
      (Effects|SpawnEmitteratLocation "/Game/VFX/P_OilExplosion.P_OilExplosion" _returnvalue)
      (Audio|PlaySoundatLocation "/Game/Audio/orbHit.orbHit" _returnvalue "0, 0, 0" 1.0 1.0 0.0 0 0 0)
      (Utilities|IsValid (Variables|Default|GetVehicleRef)
        (:Is%20Valid
          (Class|VehicleBase|SetSpeedMax (Variables|Default|GetVehicleRef) (* (Variables|/Script/TwistedMario.VehicleBase|GetspeedMax (Variables|Default|GetVehicleRef)) 1.113))
          (Class|VehicleBase|SetTurnCoefficient (Variables|Default|GetVehicleRef) (/ (Variables|/Script/TwistedMario.VehicleBase|Getturncoefficient (Variables|Default|GetVehicleRef)) 2.78))
          (if (> (Variables|/Script/TwistedMario.VehicleBase|GetspeedMax (Variables|Default|GetVehicleRef)) 1.2e+03)
            (Class|VehicleBase|SetSpeedMax (Variables|Default|GetVehicleRef) 1.2e+03)
            (if (< (Variables|/Script/TwistedMario.VehicleBase|Getturncoefficient (Variables|Default|GetVehicleRef)) 0.4)
              (Variables|/Script/TwistedMario.VehicleBase|Setturncoefficient (Variables|Default|GetVehicleRef) 0.4)))
          (Utilities|FlowControl|Delay 6.7)
          (Class|VehicleBase|SetSpeedMax (Variables|Default|GetVehicleRef) (Variables|/Script/TwistedMario.VehicleBase|GetspeedMaxOriginal (Variables|Default|GetVehicleRef)))
          (Variables|/Script/TwistedMario.VehicleBase|Setturncoefficient (Variables|Default|GetVehicleRef) (Variables|/Script/TwistedMario.VehicleBase|GetturncOriginal (Variables|Default|GetVehicleRef))))))))

(event EventBeginPlay)

(event Collision|EventActorBeginOverlap
  (params (OtherActor :type Actor%20Object%20Reference)))

(event EventTick
  (params (DeltaSeconds :type Float%20%28single-precision%29)))

(fn ConstructionScript)
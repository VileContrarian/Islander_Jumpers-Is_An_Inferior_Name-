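; Snowpile blocker that damages and temporarily slows vehicles that drive into it.
; On collider overlap with a BP_VehicleBase01, it deals damage, spawns a snow explosion and plays a hit sound at world origin.
; It halves the current max speed, with a minimum floor, then restores the original after DebuffTime.
; The comment says one third, but the code divides by two.
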(event OnComponentBeginOverlap(Collider)
  (params (OverlappedComponent :type Primitive%20Component%20Object%20Reference) (OtherActor :type Actor%20Object%20Reference) (OtherComp :type Primitive%20Component%20Object%20Reference) (OtherBodyIndex :type Integer) (bFromSweep :type Boolean) (SweepResult :type Hit%20Result%20Structure%20%28by%20ref%29))
  (bind _asvehicle_base (Utilities|Casting|CastToVehicleBase OtherActor))
  (bind _asbp_vehicle_base_01 (Utilities|Casting|CastToBP_VehicleBase01 _asvehicle_base))
  (bind _output_get (Variables|Default|SetVehicleRef _asbp_vehicle_base_01))
  (Class|VehicleBase|DoDamage _output_get 10)
  (Effects|SpawnEmitteratLocation "/Game/VFX/P_SnowExplosion.P_SnowExplosion" (Transformation|GetActorLocation))
  (Audio|PlaySoundatLocation "/Game/Audio/orbHit.orbHit" "0, 0, 0" "0, 0, 0" 1.0 1.0 0.0 0 0 0)
  (Class|VehicleBase|SetSpeedMax (Variables|Default|GetVehicleRef) (/ (Variables|/Script/TwistedMario.VehicleBase|GetspeedMax (Variables|Default|GetVehicleRef)) 2.0))
  (if (< (Variables|/Script/TwistedMario.VehicleBase|GetspeedMax (Variables|Default|GetVehicleRef)) 1e+02)
    (Class|VehicleBase|SetSpeedMax (Variables|Default|GetVehicleRef) 1e+02))
  (Utilities|FlowControl|Delay (Variables|Default|GetDebuffTime))
  ;[1 1 1 1 12] After debuff time is completed reset car's speed back to its original speed
  (Class|VehicleBase|SetSpeedMax (Variables|Default|GetVehicleRef) (Variables|/Script/TwistedMario.VehicleBase|GetspeedMaxOriginal (Variables|Default|GetVehicleRef))))

(event EventBeginPlay)

(event Collision|EventActorBeginOverlap
  (params (OtherActor :type Actor%20Object%20Reference)))

(event EventTick
  (params (DeltaSeconds :type Float%20%28single-precision%29)))

(fn ConstructionScript)
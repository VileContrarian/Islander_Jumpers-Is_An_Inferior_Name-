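; BP_Button is a menu button that keeps mouse hover and keyboard focus in sync and restyles itself to match.
; Start runs a looping timer that polls CheckFocus, and End clears it.
; Hovering takes keyboard focus and applies the mouse style; otherwise the style follows focus state.
; While focused but not hovered, each poll passes the button's Index to the game mode's PlayerSelectWidget through CallOnFocus.
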(event Custom|CallButton
  (bind _asbp_menu_game_mode (Utilities|Casting|CastToBP_MenuGameMode (Game|GetGameMode)))
  (Utilities|IsValid (Variables|/Game/Blueprints/GameModes/BP_MenuGameMode.BP_MenuGameMode_C|GetPlayerSelectWidget _asbp_menu_game_mode)
    (:Is%20Valid
      (Default|CallonFocus (Variables|/Game/Blueprints/GameModes/BP_MenuGameMode.BP_MenuGameMode_C|GetPlayerSelectWidget _asbp_menu_game_mode) (Variables|Default|Getindex)))))

(fn Start
  (bind _returnvalue (Utilities|Time|SetTimerbyFunctionName 0 "CheckFocus" 0.08 true))
  (Variables|Default|SetTimerHandle _returnvalue))

(fn CheckFocus
  (bind _returnvalue (Class|Widget|HasKeyboardFocus))
  (if (Widget|IsHovered)
    (Widget|SetKeyboardFocus)
    (Class|Button|SetStyle (Variables|Style|GetMouseStyle))
    (else
      (Class|Button|SetStyle (select _returnvalue (Variables|Style|GetKeyFocused) (Variables|Style|GetKeyNotFocused)))
      (if _returnvalue
        (CallFunction|CallButton)))))

(fn End
  (Utilities|Time|ClearandInvalidateTimerbyHandle (Variables|Default|GetTimerHandle)))
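; Level Blueprint for a four-player local character select screen where players take turns choosing.
; BeginPlay creates three extra local players, shows the BP_CharacterSelect widget and disables all controllers' input.
; A re-armed timer passes input to each controller in turn every five seconds, updating the widget's active player.
; Tick feeds a parallel twenty-second timer's progress to the widget's Completion; that timer's WaitingDone handler is empty.
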(event Custom|ChangePlayerInput
  (bind _playerselectwidget (Variables|Default|GetPlayerSelectWidget))
  ;[1 1 1] Show Character Select Menu
  (Input|DisableInput (Game|GetPlayerController (Variables|Default|GetPlayerCount)))
  (bind _result (Math|Integer|IncrementInt (Variables|Default|GetPlayerCount))
    (:%20%20
      (if (< _result 4)
        (Utilities|Time|SetTimerbyEvent (delegate Custom|ChangePlayerInput) 5.0)
        (Input|EnableInput (Game|GetPlayerController (Variables|Default|GetPlayerCount)))
        (Variables|/Game/UI/BP_CharacterSelect.BP_CharacterSelect_C|SetPlayerCount _playerselectwidget (Variables|Default|GetPlayerCount))
        (Default|ChangePlayer _playerselectwidget)))))

(event Custom|WaitingDone)

(event EventBeginPlay
  ;[1 1 1] Show Character Select Menu
  (Class|GameplayStatics|CreatePlayer -1 false)
  (Class|GameplayStatics|CreatePlayer -1 false)
  (Class|GameplayStatics|CreatePlayer -1 false)
  (bind _returnvalue (UserInterface|CreateWidget "/Game/UI/BP_CharacterSelect.BP_CharacterSelect_C"))
  (bind _output_get (Variables|Default|SetPlayerSelectWidget _returnvalue))
  (UserInterface|Viewport|AddtoViewport _output_get 0)
  (for _index (range 0 3)
    (Input|DisableInput (Game|GetPlayerController _index)))
  (bind _returnvalue_2 (Utilities|Time|SetTimerbyEvent (delegate Custom|WaitingDone) 2e+01))
  (Utilities|Time|SetTimerbyEvent (delegate Custom|ChangePlayerInput) 5.0)
  (Input|EnableInput (Game|GetPlayerController (Variables|Default|GetPlayerCount)))
  (Variables|/Game/UI/BP_CharacterSelect.BP_CharacterSelect_C|SetPlayerCount (Variables|Default|GetPlayerSelectWidget) (Variables|Default|GetPlayerCount))
  (Default|ChangePlayer (Variables|Default|GetPlayerSelectWidget)))

(event EventTick
  (params (DeltaSeconds :type Float%20%28single-precision%29))
  ;[1 1 1] EventTick Completion
  (Variables|/Game/UI/BP_CharacterSelect.BP_CharacterSelect_C|SetCompletion (Variables|Default|GetPlayerSelectWidget) (/ (Class|KismetSystemLibrary|GetTimerElapsedTimeHandle (stale EventBeginPlay _returnvalue_2)) 2e+01)))

(fn ConstructionScript)
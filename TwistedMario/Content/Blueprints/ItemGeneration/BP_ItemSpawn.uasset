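; Spawner that fills its four spot locations with random pickups or obstacles on BeginPlay.
; A single weighted roll favoring obstacles decides whether all four spots get items or obstacles, then each spot picks its class independently.
; The construction script defines both class pools, and the obstacle pool includes an empty entry.
; Obstacles spawn at reduced scale, while items spawn at full scale.
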(event EventBeginPlay
  (CallFunction|SetSpawn))

(fn ConstructionScript
  ;[1 1 1] Add Items into this array
  (Variables|Default|SetItemArray (Utilities|Array|MakeArray "/Game/Blueprints/HealthPack/BP_HealthPack_001.BP_HealthPack_001_C" "/Game/Blueprints/SpeedItems/BP_Booster.BP_Booster_C" "/Game/Blueprints/SpeedItems/BP_SpeedDown.BP_SpeedDown_C"))
  ;[1 1 1] Add Obstacles into this array
  (Variables|Default|SetObstacleArray (Utilities|Array|MakeArray "/Game/Blueprints/Blockers/BL_Snowpile.BL_Snowpile_C" "/Game/Blueprints/Blockers/BL_Rock.BL_Rock_C" "/Game/Blueprints/Blockers/BL_Oil.BL_Oil_C" 0)))

(fn SetSpawn
  (if (< (Math|Random|RandomIntegerinRange 1 10) 5)
    (Variables|Default|SetisSpawningItem true)
    (else
      (Variables|Default|SetisSpawningItem false)))
  (bind _output_get (Variables|Default|SetSpawnPositionArray (Utilities|Array|MakeArray (Transformation|GetWorldLocation (Variables|Default|GetSpotA)) (Transformation|GetWorldLocation (Variables|Default|GetSpotB)) (Transformation|GetWorldLocation (Variables|Default|GetSpotC)) (Transformation|GetWorldLocation (Variables|Default|GetSpotD)))))
  (for _index (range 0 (Utilities|Array|LastIndex _output_get))
    (if (Variables|Default|GetisSpawningItem)
      (bind _returnitem (CallFunction|RandomizeItems))
      (Game|SpawnActorfromClass _returnitem (Math|Transform|MakeTransform (Utilities|Array|Get(acopy) _output_get _index)) "Undefined" 0 0)
      (else
        (bind _returnobstacle (CallFunction|RandomizeObstacles))
        (Game|SpawnActorfromClass _returnobstacle (Math|Transform|MakeTransform (Utilities|Array|Get(acopy) _output_get _index) "0, 0, 0" "0.400000,0.400000,0.400000") "Undefined" 0 0)))))

(fn RandomizeItems
  (bind _itemarray (Variables|Default|GetItemArray))
  (return (Utilities|Array|Get(acopy) _itemarray (Math|Random|RandomIntegerinRange 0 (Utilities|Array|LastIndex _itemarray)))))

(fn RandomizeObstacles
  (bind _obstaclearray (Variables|Default|GetObstacleArray))
  (return (Utilities|Array|Get(acopy) _obstaclearray (Math|Random|RandomIntegerinRange 0 (Utilities|Array|LastIndex _obstaclearray)))))
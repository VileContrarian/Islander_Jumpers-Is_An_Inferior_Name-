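; BP_WarpPoint is a warp trigger for vehicles that records entry data, leaving the warp implementation to the level Blueprint.
; When a BP_VehicleBase01 begins overlapping the Warp component, it sets an entering flag and stores the vehicle.
; It also saves the car body's position offset from Warp and its speed as a scalar.
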(event OnComponentBeginOverlap(Warp)
  (params (OverlappedComponent :type Primitive%20Component%20Object%20Reference) (OtherActor :type Actor%20Object%20Reference) (OtherComp :type Primitive%20Component%20Object%20Reference) (OtherBodyIndex :type Integer) (bFromSweep :type Boolean) (SweepResult :type Hit%20Result%20Structure%20%28by%20ref%29))
  ;[1 1 1] I'm only storing values in this object. The implementation is in the level BP.
  (bind _asbp_vehicle_base_01 (Utilities|Casting|CastToBP_VehicleBase01 OtherActor))
  (Variables|Default|SetisEntering true)
  (Variables|Default|SetVehicleObject _asbp_vehicle_base_01)
  (Variables|Default|SetEntryLocation (- (Transformation|GetWorldLocation (Variables|/Game/Blueprints/VehicleBase/BP_VehicleBase01.BP_VehicleBase01_C|GetCarBody _asbp_vehicle_base_01)) (Transformation|GetWorldLocation (Variables|Default|GetWarp))))
  (Variables|Default|SetEntrySpeed (Math|Vector|VectorLength (Transformation|GetComponentVelocity (Variables|/Game/Blueprints/VehicleBase/BP_VehicleBase01.BP_VehicleBase01_C|GetCarBody _asbp_vehicle_base_01)))))

(event EventBeginPlay)

(event EventTick
  (params (DeltaSeconds :type Float%20%28single-precision%29)))

(fn ConstructionScript)
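; Game mode for a local multiplayer vehicle race, running setup, countdown and finish check.
; BeginPlay reads player count, laps and vehicle classes from BP_GameInfoInstance, spawns players at tagged PlayerStarts, and enables input after the countdown.
; It handles damage, healing and kills with timed respawns; Tick calls EndGame, which only prints, once all players finish.
; UpdatePositions derives race placings from summed map, lap and checkpoint indices, but nothing here calls it.
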(event Custom|Respawn
  (bind _lastrespawnpoint (Default|GetRespawnPoint (stale Custom|Kill _asbp_vehicle_controller)))
  (bind _returnvalue (Game|SpawnActorfromClass (Utilities|GetClass (Pawn|GetControlledPawn (stale Custom|Kill _asbp_vehicle_controller))) _lastrespawnpoint "AdjustIfPossibleButDontSpawnIfColliding" 0 0))
  (Class|PlayerController|SetCinematicMode (stale Custom|Kill _asbp_vehicle_controller) false false false true true)
  (Pawn|Possess (stale Custom|Kill _asbp_vehicle_controller) _returnvalue))

(event Custom|Kill
  (params (PlayerController :type Player%20Controller%20Object%20Reference%20%28by%20ref%29))
  (bind _asbp_vehicle_controller (Utilities|Casting|CastToBP_VehicleController PlayerController))
  (Actor|DestroyActor (Pawn|GetControlledPawn _asbp_vehicle_controller))
  (Pawn|UnPossess _asbp_vehicle_controller)
  (Class|PlayerController|SetCinematicMode _asbp_vehicle_controller true false false true true)
  (Utilities|Time|SetTimerbyEvent (delegate Custom|Respawn) 2.0))

(event Custom|EndGame
  (Development|PrintString "Game Ended"))

(event Custom|Damage
  (params (DamageFrom :type BP%20Vehicle%20Controller%20Object%20Reference%20%28by%20ref%29) (DamageTo :type BP%20Vehicle%20Controller%20Object%20Reference%20%28by%20ref%29) (Amount :type Integer))
  (bind _asbp_vehicle_base_01 (Utilities|Casting|CastToBP_VehicleBase01 (Pawn|GetControlledPawn DamageTo)))
  (Utilities|IsValid _asbp_vehicle_base_01
    (:Is%20Valid
      (Class|VehicleBase|DoDamage _asbp_vehicle_base_01 Amount))))

(event Custom|Heal
  (params (Player :type BP%20Vehicle%20Controller%20Object%20Reference%20%28by%20ref%29) (Amount :type Integer%20%28by%20ref%29))
  (bind _asbp_vehicle_base_01 (Utilities|Casting|CastToBP_VehicleBase01 (Pawn|GetControlledPawn Player)))
  (Utilities|IsValid _asbp_vehicle_base_01
    (:Is%20Valid
      (Class|VehicleBase|DoHeal _asbp_vehicle_base_01 Amount))))

(event Custom|GameStart
  (Development|PrintString "On your marks")
  (Utilities|FlowControl|Delay 1.0)
  (Development|PrintString "3")
  (Utilities|FlowControl|Delay 1.0)
  (Development|PrintString "2")
  (Utilities|FlowControl|Delay 1.0)
  (Development|PrintString "1")
  (Utilities|FlowControl|Delay 1.0)
  (Development|PrintString "GO!")
  (for (_ _array_index) (Variables|Default|GetPlayers)
    (bind _asbp_vehicle_controller (Utilities|Casting|CastToBP_VehicleController (Game|GetPlayerController _array_index)))
    (Input|EnableInput _asbp_vehicle_controller _asbp_vehicle_controller)))

(event EventBeginPlay
  (CallFunction|LoadValuesfromInstance)
  (CallFunction|GetPlayerStartPoints)
  (CallFunction|SpawnPlayers)
  (Utilities|FlowControl|Delay 2.0)
  (CallFunction|GameStart))

(event EventTick
  (params (DeltaSeconds :type Float%20%28single-precision%29))
  (CallFunction|CheckGameStatus))

(fn ConstructionScript)

(fn UpdatePositions
  (bind _positions (Variables|Default|GetPositions))
  ;[1 1 1] Comment
  (for _index (range 0 (Variables|Default|GetCurrentNumPlayers))
    (bind _asbp_vehicle_controller (Utilities|Casting|CastToBP_VehicleController (Game|GetPlayerController _index)))
    (LocalVariables|SetVehicleController _asbp_vehicle_controller)
    (if (Utilities|Map|Contains (Variables|Default|GetPositions) (+ (Variables|/Game/Blueprints/GamePlayerControllers/BP_VehicleController.BP_VehicleController_C|GetCurrentMapIndex _asbp_vehicle_controller) (Variables|/Game/Blueprints/GamePlayerControllers/BP_VehicleController.BP_VehicleController_C|GetLapIndex _asbp_vehicle_controller) (Variables|/Game/Blueprints/GamePlayerControllers/BP_VehicleController.BP_VehicleController_C|GetLastCheckpointIndex _asbp_vehicle_controller)))
      (bind _result (Math|Integer|IncrementInt (+ (Variables|/Game/Blueprints/GamePlayerControllers/BP_VehicleController.BP_VehicleController_C|GetCurrentMapIndex _asbp_vehicle_controller) (Variables|/Game/Blueprints/GamePlayerControllers/BP_VehicleController.BP_VehicleController_C|GetLapIndex _asbp_vehicle_controller) (Variables|/Game/Blueprints/GamePlayerControllers/BP_VehicleController.BP_VehicleController_C|GetLastCheckpointIndex _asbp_vehicle_controller)))
        (:%20%20
          (Utilities|Map|Add _positions _result (LocalVariables|GetVehicleController))))
      (else
        (Utilities|Map|Add _positions (+ (Variables|/Game/Blueprints/GamePlayerControllers/BP_VehicleController.BP_VehicleController_C|GetCurrentMapIndex _asbp_vehicle_controller) (Variables|/Game/Blueprints/GamePlayerControllers/BP_VehicleController.BP_VehicleController_C|GetLapIndex _asbp_vehicle_controller) (Variables|/Game/Blueprints/GamePlayerControllers/BP_VehicleController.BP_VehicleController_C|GetLastCheckpointIndex _asbp_vehicle_controller)) (LocalVariables|GetVehicleController)))))
  (bind _keys (Utilities|Map|Keys (Variables|Default|GetPositions)))
  (for (_array_element _array_index) _keys
    (Development|PrintString (Utilities|String|Append (Utilities|String|ToString(Integer) _array_index) "\":\\t\"" (Utilities|String|ToString(Integer) _array_element)))
    (if (.ReturnValue (Utilities|Map|Find (Variables|Default|GetPositions) _array_element))
      (bind _result_2 (Math|Integer|IncrementInt _array_index)
        (:%20%20
          (Variables|/Game/Blueprints/GamePlayerControllers/BP_VehicleController.BP_VehicleController_C|SetPositionIndex (.Value (Utilities|Map|Find (Variables|Default|GetPositions) _array_element)) _result_2)))))
  (Utilities|Map|Clear (Variables|Default|GetPositions)))

(fn GetPlayerStartPoints
  (bind _outactors (Actor|GetAllActorsOfClass "/Script/Engine.PlayerStart"))
  (Variables|Default|SetPlayerStartArray _outactors))

(fn SpawnPlayers
  (for _index (range 0 (- (Variables|Default|GetCurrentNumPlayers) 1))
    (LocalVariables|SetIndex _index)
    (for _array_element (Variables|Default|GetPlayerStartArray)
      (if (Utilities|Name|Equal(Name) (Variables|/Script/Engine.PlayerStart|GetPlayerStartTag _array_element) (Utilities|String|StringToName (Utilities|String|ToString(Integer) (LocalVariables|GetIndex))))
        (Class|GameplayStatics|CreatePlayer (LocalVariables|GetIndex) false)
        (bind _asbp_vehicle_controller (Utilities|Casting|CastToBP_VehicleController (Game|GetPlayerController (LocalVariables|GetIndex))))
        (if (.ReturnValue (Utilities|Map|Find (Variables|Default|GetPlayerTypes) (LocalVariables|GetIndex)))
          (bind _returnvalue (Game|SpawnActorfromClass (.Value (Utilities|Map|Find (Variables|Default|GetPlayerTypes) (LocalVariables|GetIndex))) (Transformation|GetActorTransform _array_element) "AdjustIfPossibleButAlwaysSpawn" 0 0))
          (Pawn|Possess _asbp_vehicle_controller _returnvalue)
          (Utilities|Array|AddUnique (Variables|Default|GetPlayers) _returnvalue)
          (Input|DisableInput _asbp_vehicle_controller _asbp_vehicle_controller)
          (else
            (bind _returnvalue_2 (Game|SpawnActorfromClass "/Game/GameContent/BP_VehicleBase01.BP_VehicleBase01_C" (Transformation|GetActorTransform _array_element) "AdjustIfPossibleButAlwaysSpawn" 0 0))
            (Pawn|Possess _asbp_vehicle_controller _returnvalue_2)
            (Utilities|Array|AddUnique (Variables|Default|GetPlayers) _returnvalue_2)
            (Input|DisableInput _asbp_vehicle_controller _asbp_vehicle_controller)))))))

(fn LoadValuesfromInstance
  (bind _asbp_game_info_instance (Utilities|Casting|CastToBP_GameInfoInstance (Game|GetGameInstance)))
  (bind _output_get (LocalVariables|SetInstance _asbp_game_info_instance))
  (Variables|Default|SetCurrentNumPlayers (Variables|/Game/Blueprints/GameInstances/BP_GameInfoInstance.BP_GameInfoInstance_C|GetPlayerCount _output_get))
  (Variables|Default|SetNumLaps (Variables|/Game/Blueprints/GameInstances/BP_GameInfoInstance.BP_GameInfoInstance_C|GetNumberofLaps (LocalVariables|GetInstance)))
  (Variables|Default|SetPlayerTypes (Variables|/Game/Blueprints/GameInstances/BP_GameInfoInstance.BP_GameInfoInstance_C|GetPlayers (LocalVariables|GetInstance))))

(fn CheckGameStatus
  ;[1 1 1] Loop Through All Player Controller To Check if they have finished else break
  (bind _index (Utilities|FlowControl|ForLoopwithBreak 0 (- (Variables|Default|GetCurrentNumPlayers) 1) :!label _label)
    (:LoopBody
      (bind _asbp_vehicle_controller (Utilities|Casting|CastToBP_VehicleController (Game|GetPlayerController _index)))
      (if (Math|Boolean|Equal(Boolean) true (Variables|/Game/Blueprints/GamePlayerControllers/BP_VehicleController.BP_VehicleController_C|GetIsFinished _asbp_vehicle_controller))
        (Variables|Default|SetHasGameEnded true)
        (else
          (Variables|Default|SetHasGameEnded false)
          (goto _label Break))))
    (:Completed
      (if (Variables|Default|GetHasGameEnded)
        (CallFunction|EndGame)))))
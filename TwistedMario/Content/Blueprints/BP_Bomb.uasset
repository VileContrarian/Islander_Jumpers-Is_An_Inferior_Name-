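; Timed bomb actor that damages and knocks back vehicles and destroys rock, snowpile and pillar obstacles in its blast.
; Tick decrements a frame-based timer; at zero it expands a sphere collider to blast radius and plays effects, then destroys itself at -1.
; Overlap events raised while Exploded is true apply damage and add outward velocity to vehicle meshes, or destroy obstacles.
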(event OnComponentBeginOverlap(ExplosionCollider)
  (params (OverlappedComponent :type Primitive%20Component%20Object%20Reference) (OtherActor :type Actor%20Object%20Reference) (OtherComp :type Primitive%20Component%20Object%20Reference) (OtherBodyIndex :type Integer) (bFromSweep :type Boolean) (SweepResult :type Hit%20Result%20Structure%20%28by%20ref%29))
  ;[1 1 1] If exploded=true call Explode
  (if (Variables|Default|GetExploded)
    (bind _asvehicle_base (Utilities|Casting|CastToVehicleBase OtherActor)
      (:then
        (CallFunction|Explode _asvehicle_base))
      (:CastFailed
        ;[1 1 1] Destroy basic obstacles if caught within blast radius (experimental)
        (bind _asbl_rock (Utilities|Casting|CastToBL_Rock OtherActor)
          (:then
            (Actor|DestroyActor _asbl_rock))
          (:CastFailed
            (bind _asbl_snowpile (Utilities|Casting|CastToBL_Snowpile OtherActor)
              (:then
                (Actor|DestroyActor _asbl_snowpile))
              (:CastFailed
                (bind _asbl_pillar (Utilities|Casting|CastToBL_Pillar OtherActor))
                (Actor|DestroyActor _asbl_pillar)))))))))

(event EventTick
  (params (DeltaSeconds :type Float%20%28single-precision%29))
  (bind _bombmesh (Variables|Default|GetBombMesh))
  (bind _returnvalue (Transformation|GetWorldLocation _bombmesh))
  ;[1 1 1] Timer countdown to explosion
  (bind _result (Math|Integer|DecrementInt (Variables|Default|GetTimer))
    (:%20%20
      (bind _output_get (Variables|Default|SetTimer _result))
      (bind _output_get_2 (Variables|Default|SetExploded (== _output_get 0)))
      (if _output_get_2
        ;[1 1 1] Expand to explosion radius
        (Components|Sphere|SetSphereRadius (Variables|Default|GetExplosionCollider) (Variables|Default|GetExplosion%20Radius) true)
        ;[1 1 1] Explosion FX
        (bind _returnvalue_2 (Effects|SpawnEmitteratLocation "/Game/VFX/FX_BombExplosion.FX_BombExplosion" _returnvalue "0, 0, 0" "7.000000,7.000000,7.000000"))
        (Audio|PlaySoundatLocation "/Game/Audio/Amb_Explosion.Amb_Explosion" _returnvalue "0, 0, 0" 1.0 1.0 0.0 0 0 0)
        (Utilities|FlowControl|Delay 0.8)
        (Components|DestroyComponent _returnvalue_2)
        (else
          ;[1 1 1] Destroy self 1s after explosion
          (if (== (Variables|Default|GetTimer) -1)
            (Actor|DestroyActor)))))))

(fn ConstructionScript)

(fn Explode
  (params (OverlappedVehicle :type Vehicle%20Base%20Object%20Reference))
  ;[1 1 1] Deal damage, Puch vehicle
  (Class|VehicleBase|DoDamage OverlappedVehicle (Variables|Default|GetDamageToDeal))
  (CallFunction|PushVehicle OverlappedVehicle))

(fn PushVehicle
  (params (OverlappedVehicle :type Vehicle%20Base%20Object%20Reference))
  ;[1 1 1] Get direction vector and multiply by explosion force
  (Physics|SetPhysicsLinearVelocity (Variables|/Script/TwistedMario.VehicleBase|GetCarMesh OverlappedVehicle) (* (Math|Vector|Normalize (- (Transformation|GetActorLocation OverlappedVehicle) (Transformation|GetWorldLocation (Variables|Default|GetBombMesh)))) (Variables|Default|GetExplosionForce)) true "None"))
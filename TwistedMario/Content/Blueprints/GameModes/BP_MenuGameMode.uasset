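; Menu game mode that spawns the front-end widgets, from title card to placements, and runs player join and timed character select.
; Join counts active BP_MenuController players into BP_GameInfoInstance, which sets how many local players character select creates.
; Character select gives each player a timed turn, using cinematic mode to lock the others' input and Tick to update widget progress.
; An override can end a turn early; when turns finish, it removes the players and opens MainGameLevel.
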(event Custom|DisplayMainMenu
  ;[0 1 0.455] Creation
  ;;[1 1 1] Creating & Adding Main Menu
  (bind _returnvalue (UserInterface|CreateWidget "/Game/UI/BP_MainMenu.BP_MainMenu_C"))
  (UserInterface|Viewport|AddtoViewport _returnvalue 0))

(event Custom|DisplayPlayTypeMenu
  ;[0 1 0.455] Creation
  ;;[1 1 1] Creating & Adding Play Type Menu
  (bind _returnvalue (UserInterface|CreateWidget "/Game/UI/BP_PlayType.BP_PlayType_C"))
  (UserInterface|Viewport|AddtoViewport _returnvalue 0))

(event Custom|DisplayTitleCard
  ;[0 1 0.455] Creation
  ;;[1 1 1] Creating & Adding TitleCard
  (bind _returnvalue (UserInterface|CreateWidget "/Game/UI/TitleCard_BP.TitleCard_BP_C"))
  (UserInterface|Viewport|AddtoViewport _returnvalue 0))

(event Custom|ChangePlayerInputOverride
  (bind _currentplayertimer (Variables|Default|GetCurrentPlayerTimer))
  ;[0.4445 1 0] Functionality
  ;;[1 1 1] Change Player Input Override
  (Utilities|Time|ClearandInvalidateTimerbyHandle _currentplayertimer)
  (Utilities|Time|ClearandInvalidateTimerbyHandle (Variables|Default|GetPlayerSelectTotalTimer))
  (bind _returnvalue (Utilities|Time|SetTimerbyEvent (delegate Custom|WaitingDone) (- (Utilities|Time|GetTimerRemainingTimebyHandle (Variables|Default|GetPlayerSelectTotalTimer)) (Utilities|Time|GetTimerRemainingTimebyHandle _currentplayertimer))))
  (Variables|Default|SetPlayerSelectTotalTimer _returnvalue)
  (CallFunction|ChangePlayerInput))

(event Custom|DisplayPlacementsMenu
  ;[0 1 0.455] Creation
  ;;[1 1 1] Creating & Adding Placements Menu
  (bind _returnvalue (UserInterface|CreateWidget "/Game/UI/BP_Placements.BP_Placements_C"))
  (UserInterface|Viewport|AddtoViewport _returnvalue 0))

(event Custom|DisplayCreditEvent
  (bind _returnvalue (UserInterface|CreateWidget "/Game/UI/BP_Credits.BP_Credits_C"))
  (UserInterface|Viewport|AddtoViewport _returnvalue 0))

(event Custom|DisplayOptionsMenu
  ;[0 1 0.455] Creation
  ;;[1 1 1] Creating & Adding Options Menu
  (bind _returnvalue (UserInterface|CreateWidget "/Game/UI/BP_OptionsMenu.BP_OptionsMenu_C"))
  (UserInterface|Viewport|AddtoViewport _returnvalue 0))

(event Custom|DisplayCharacterSelectMenu
  ;[0 1 0.455] Creation
  ;;[1 1 1] Creating & Adding Player Select Menu
  (bind _returnvalue (UserInterface|CreateWidget "/Game/UI/BP_CharacterSelect.BP_CharacterSelect_C"))
  (bind _output_get (Variables|Default|SetPlayerSelectWidget _returnvalue))
  (UserInterface|Viewport|AddtoViewport _output_get 0))

(event Custom|PlayerSelectStart
  ;[0.4445 1 0] Functionality
  ;;[1 1 1] Starting Player Select Menu
  (Variables|Default|SetInPlayerSelect true)
  (CallFunction|SetUpCamera)
  (CallFunction|CreatePlayers (Variables|/Game/Blueprints/GameInstances/BP_GameInfoInstance.BP_GameInfoInstance_C|GetPlayerCount (Variables|Default|GetGameInstance)))
  (CallFunction|DisplayCharacterSelectMenu)
  (CallFunction|DisableAllPlayersInput)
  (bind _returnvalue (Utilities|Time|SetTimerbyEvent (delegate Custom|WaitingDone) (* (Variables|/Game/Blueprints/GameInstances/BP_GameInfoInstance.BP_GameInfoInstance_C|GetPlayerCount (Variables|Default|GetGameInstance)) (Variables|Default|GetTimePerPlayer))))
  (Variables|Default|SetPlayerSelectTotalTimer _returnvalue)
  (Variables|Default|SetCanStartCountdown true)
  (CallFunction|SetPlayerTimer))

(event Custom|DisplayPlayerJoinMenu
  ;[0 1 0.455] Creation
  ;;[1 1 1] Creating & Adding Player Join Menu
  (bind _returnvalue (UserInterface|CreateWidget "/Game/UI/BP_PlayerJoin.BP_PlayerJoin_C"))
  (bind _output_get (Variables|Default|SetPlayer%20Join%20Widget _returnvalue))
  (UserInterface|Viewport|AddtoViewport _output_get 0)
  (Class|GameplayStatics|CreatePlayer (Variables|/Game/Blueprints/GameInstances/BP_GameInfoInstance.BP_GameInfoInstance_C|GetMaxPlayerCount (Variables|Default|GetGameInstance))))

(event Custom|UpdatePlayerCount
  (bind _gameinstance (Variables|Default|GetGameInstance))
  (bind _maxplayercount (Variables|/Game/Blueprints/GameInstances/BP_GameInfoInstance.BP_GameInfoInstance_C|GetMaxPlayerCount _gameinstance))
  ;[0.4445 1 0] Functionality
  ;;[1 1 1] Update Player Count Event
  (Variables|/Game/Blueprints/GameInstances/BP_GameInfoInstance.BP_GameInfoInstance_C|SetPlayerCount _gameinstance 0)
  (Utilities|Array|Resize (Variables|Default|GetPlayerActiveArray) _maxplayercount)
  (for _index (range 0 (- _maxplayercount 1))
    (bind _asbp_menu_controller (Utilities|Casting|CastToBP_MenuController (Game|GetPlayerController _index)))
    (Utilities|Array|SetArrayElem (Variables|Default|GetPlayerActiveArray) _index (Variables|/Game/Blueprints/GamePlayerControllers/BP_MenuController.BP_MenuController_C|GetActive _asbp_menu_controller)))
  (for _array_element (Variables|Default|GetPlayerActiveArray)
    (if _array_element
      (Math|Integer|IncrementInt (Variables|/Game/Blueprints/GameInstances/BP_GameInfoInstance.BP_GameInfoInstance_C|GetPlayerCount (Variables|Default|GetGameInstance)))))
  (Default|UpdatePlayerTotal (Variables|Default|GetPlayer%20Join%20Widget)))

(event Custom|ChangePlayerInput
  (bind _playerselectwidget (Variables|Default|GetPlayerSelectWidget))
  ;[0.4445 1 0] Functionality
  ;;[1 1 1] Disabling Current Player Input and Enabling Next One
  (Utilities|IsValid (Game|GetPlayerController (Variables|Default|GetPlayerIndex))
    (:Is%20Valid
      (Class|PlayerController|SetCinematicMode (Game|GetPlayerController (Variables|Default|GetPlayerIndex)) true false false false false)
      (bind _result (Math|Integer|IncrementInt (Variables|Default|GetPlayerIndex))
        (:%20%20
          (if (< _result (Variables|/Game/Blueprints/GameInstances/BP_GameInfoInstance.BP_GameInfoInstance_C|GetPlayerCount (Variables|Default|GetGameInstance)))
            ;;[1 1 1] Setting Individual Player Timer. Allowing Access to Individual Player
            (bind _returnvalue (Utilities|Time|SetTimerbyEvent (delegate Custom|ChangePlayerInput) (Variables|Default|GetTimePerPlayer)))
            (Variables|Default|SetCurrentPlayerTimer _returnvalue)
            (Class|PlayerController|SetCinematicMode (Game|GetPlayerController (Variables|Default|GetPlayerIndex)) false false false false false)
            (Variables|/Game/UI/BP_CharacterSelect.BP_CharacterSelect_C|SetPlayerIndex _playerselectwidget (Variables|Default|GetPlayerIndex))
            (Default|ChangePlayer _playerselectwidget)
            (else
              (CallFunction|WaitingDone))))))
    (:Is%20Not%20Valid
      (CallFunction|WaitingDone))))

(event Custom|SetPlayerTimer
  (bind _playerselectwidget (Variables|Default|GetPlayerSelectWidget))
  ;[0.4445 1 0] Functionality
  ;;[1 1 1] Setting Individual Player Timer. Allowing Access to Individual Player
  (bind _returnvalue (Utilities|Time|SetTimerbyEvent (delegate Custom|ChangePlayerInput) (Variables|Default|GetTimePerPlayer)))
  (Variables|Default|SetCurrentPlayerTimer _returnvalue)
  (Class|PlayerController|SetCinematicMode (Game|GetPlayerController (Variables|Default|GetPlayerIndex)) false false false false false)
  (Variables|/Game/UI/BP_CharacterSelect.BP_CharacterSelect_C|SetPlayerIndex _playerselectwidget (Variables|Default|GetPlayerIndex))
  (Default|ChangePlayer _playerselectwidget))

(event Custom|WaitingDone
  ;[0.4445 1 0] Functionality
  ;;[1 1 1] TO DO: Once the Player Timer is Done Load the Game
  (Widget|RemovefromParent (Variables|Default|GetPlayerSelectWidget))
  (CallFunction|DestroyPlayers (Variables|/Game/Blueprints/GameInstances/BP_GameInfoInstance.BP_GameInfoInstance_C|GetPlayerCount (Variables|Default|GetGameInstance)))
  (Game|OpenLevel(byName) "MainGameLevel")
  (Variables|Default|SetInPlayerSelect false))

(event EventBeginPlay
  ;[0 1 0.455] Creation
  ;;[1 1 1] Event Begin Play Retrieving Game Instance
  (bind _asbp_game_info_instance (Utilities|Casting|CastToBP_GameInfoInstance (Game|GetGameInstance)))
  (Variables|Default|SetGameInstance _asbp_game_info_instance))

(event EventTick
  (params (DeltaSeconds :type Float%20%28single-precision%29))
  ;[0.4445 1 0] Functionality
  ;;[1 1 1] Updating Completion for UI
  (if (Variables|Default|GetCanStartCountdown)
    (Variables|/Game/UI/BP_CharacterSelect.BP_CharacterSelect_C|SetCompletion (Variables|Default|GetPlayerSelectWidget) (/ (Class|KismetSystemLibrary|GetTimerElapsedTimeHandle (Variables|Default|GetPlayerSelectTotalTimer)) (* (Variables|/Game/Blueprints/GameInstances/BP_GameInfoInstance.BP_GameInfoInstance_C|GetPlayerCount (Variables|Default|GetGameInstance)) (Variables|Default|GetTimePerPlayer))))))

(fn ConstructionScript)

(fn SetUpCamera
  (Game|Player|SetViewTargetwithBlend (Game|GetPlayerController 0) (Variables|Camera|GetPlayerSelectCamera) 0.0 "VTBlend_Linear" 0.0 false))

(fn CreatePlayers
  (params (PlayerCount :type Integer))
  (for _index (range 0 (- PlayerCount 1))
    (Class|GameplayStatics|CreatePlayer _index false)
    (Development|PrintString (Utilities|String|Append "Created Player " (Utilities|String|ToString(Integer) _index)) true true "(R=0.000000,G=1.000000,B=0.250000,A=1.000000)")))

(fn DisableAllPlayersInput
  (for _index (range 0 3)
    (Utilities|IsValid (Game|GetPlayerController _index)
      (:Is%20Valid
        (Class|PlayerController|SetCinematicMode (Game|GetPlayerController _index) true false false false false)))))

(fn DestroyPlayers
  (params (PlayerCount :type Integer))
  (for _index (range 0 (- PlayerCount 1))
    (Class|GameplayStatics|RemovePlayer (Game|GetPlayerController _index) false)))

(fn GetPlayerType
  ;[1 1 1] Selects And Assigns Vehicle to player index
  (for (_array_element _array_index) (Variables|/Game/UI/BP_CharacterSelect.BP_CharacterSelect_C|GetPlayerCharacters (Variables|Default|GetPlayerSelectWidget))
    (switch int _array_element
      (:Default
        _)
      (:0
        _)
      (:1
        _)
      (:2
        _)
      (:3
        _)
      (:4
        _))
    (Utilities|Map|Add (Variables|/Game/Blueprints/GameInstances/BP_GameInfoInstance.BP_GameInfoInstance_C|GetPlayers (Variables|Default|GetGameInstance)) _array_index 0)))
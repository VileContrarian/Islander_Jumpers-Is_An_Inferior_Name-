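; Game mode that spawns and assigns vehicles to players as they join a vehicle game.
; On server PostLogin it increments the player count, finds the PlayerStart tagged with that number, spawns the car class indexed by the game instance's first CarIndex entry, and possesses it.
; A separate local-play function creates players with a fixed vehicle class at tagged starts, but nothing here calls it.
; Debug prints trace the login flow.
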(event EventBeginPlay)

(event EventPostLogin
  (params (NewPlayer :type Player%20Controller%20Object%20Reference))
  (Networking|SwitchHasAuthority
    (:Authority
      ;[1 1 1] Debugging Purposes
      (Development|PrintString (Utilities|GetDisplayName NewPlayer) true true "(R=1.000000,G=0.126427,B=0.246205,A=1.000000)" 6e+01)
      ;[1 1 1] Sets Necessary Variables then Spawns Players
      (OnlinePlay|SetOnlineVariables NewPlayer)
      (OnlinePlay|SpawnPlayersOnlinePlay) ; Spawns A Vehicle and GIves A Pawn to Controller
      ;[1 1 1] Removes UI Controls and Removes Mouse from Screen
      (Input|SetInputModeGameOnly NewPlayer)
      (Variables|/Script/Engine.PlayerController|SetbShowMouseCursor NewPlayer false))
    (:Remote
      (Development|PrintString "Hello" true true "(R=0.000000,G=0.660000,B=1.000000,A=1.000000)" 6e+01))))

(fn ConstructionScript)

(fn SpawnPlayersLocalPlay
  (for _index (range 0 (Variables|LocalPlayerRelated|GetNumberOfPlayers))
    (Variables|LocalandOnlinePlayerRelated|SetPlayerCount _index)
    (for _array_element (Variables|PlayerSpawnPoints|GetPlayersStarts_Array)
      ;[1 1 1] Creates a Player and Spawns Vehicle
      (if (Utilities|Name|Equal(Name) (Variables|/Script/Engine.PlayerStart|GetPlayerStartTag _array_element) (Utilities|String|StringToName (Utilities|String|ToString(Integer) (Variables|LocalandOnlinePlayerRelated|GetPlayerCount))))
        (Class|GameplayStatics|CreatePlayer (Variables|LocalandOnlinePlayerRelated|GetPlayerCount))
        (bind _returnvalue (Game|SpawnActorfromClass "/Game/Blueprints/VehicleBase/BP_VehicleBase01.BP_VehicleBase01_C" (Transformation|GetActorTransform _array_element) "Undefined" 0 0))
        (Pawn|Possess (Game|GetPlayerController (Variables|LocalandOnlinePlayerRelated|GetPlayerCount)) _returnvalue)))))

(fn SetPlayerStartPointsVariables
  (bind _outactors (Actor|GetAllActorsOfClass "/Script/Engine.PlayerStart"))
  (Variables|PlayerSpawnPoints|SetPlayersStarts_Array _outactors))

(fn SpawnPlayersOnlinePlay
  ;[1 1 1] To Be Used independently from SpawnPlayersLocalPlay and SetPlayersStartPointsVariables
  ;;[1 1 1] Itterates through Players to Find Appropriate Spawn Location
  (for _array_element (Variables|PlayerSpawnPoints|GetPlayersStarts_Array)
    (if (Utilities|Name|Equal(Name) (Variables|/Script/Engine.PlayerStart|GetPlayerStartTag _array_element) (Utilities|String|StringToName (Utilities|String|ToString(Integer) (Variables|LocalandOnlinePlayerRelated|GetPlayerCount))))
      ;;[1 1 1] Deubgging Purposes
      (Development|PrintString (Utilities|GetDisplayName _array_element) true true "(R=0.626132,G=0.012887,B=1.000000,A=1.000000)" 6e+01)
      (OnlinePlay|SpawnandPossessOnline (Transformation|GetActorTransform _array_element))
      (Development|PrintString "Hello" true true "(R=1.000000,G=0.461584,B=0.113665,A=1.000000)" 6e+01))))

(fn SetOnlineVariables
  (params (Player%20Controller%20Ref :type Player%20Controller%20Object%20Reference))
  ;[1 1 1] Do we have Player Controller?
  (Utilities|IsValid Player%20Controller%20Ref
    (:Is%20Valid
      ;[1 1 1] Sets "Player Spawn Points" & "Local and online Player Related" Variables
      (bind _output_get (Variables|LocalandOnlinePlayerRelated|SetPlayerControllerRef Player%20Controller%20Ref)) ; Set's Player Controller Reference
      (bind _outactors (Actor|GetAllActorsOfClass "/Script/Engine.PlayerStart")) ; Get's all Player Starting Points
      (Variables|LocalandOnlinePlayerRelated|SetPlayerCount (+ (Variables|LocalandOnlinePlayerRelated|GetPlayerCount) 1)) ; Increments the Count of How Mnay Players Are In Game
      (Variables|PlayerSpawnPoints|SetPlayersStarts_Array _outactors)
      (Development|PrintString (Utilities|String|Append "At Login: PlayerCount" (Utilities|String|ToString(Integer) (+ (Variables|LocalandOnlinePlayerRelated|GetPlayerCount) 1))) true true "(R=0.000000,G=0.660000,B=1.000000,A=1.000000)" 6e+01))))

(fn SpawnandPossessOnline
  (params (SpawnLocation :type Transform))
  (bind _playercontrollerref (Variables|LocalandOnlinePlayerRelated|GetPlayerControllerRef))
  (bind _asbp_game_info_instance (Utilities|Casting|CastToBP_GameInfoInstance (Game|GetGameInstance)))
  (bind _returnvalue (Game|SpawnActorfromClass (Utilities|Array|Get(acopy) (Variables|Default|GetCarClass) (Utilities|Array|Get(acopy) (Variables|/Game/Blueprints/BPD_CarInformation.BPD_CarInformation_C|GetCarIndex (Variables|/Game/Blueprints/GameInstances/BP_GameInfoInstance.BP_GameInfoInstance_C|GetCarInfoRef _asbp_game_info_instance)))) SpawnLocation "Undefined" 0 0)) ; Spawns Vehicle at Matching Spawn Location
  (bind _asvehicle_base (Utilities|Casting|CastToVehicleBase _returnvalue))
  (Pawn|Possess _playercontrollerref _asvehicle_base)
  ;[1 1 1] Prints Out Player Spawn Location Alongside The Player Controller
  (Development|PrintString (Utilities|String|Append "At Login: Possessed" (Utilities|GetDisplayName _playercontrollerref)) true true "(R=0.000000,G=0.658824,B=1.000000,A=1.000000)" 6e+01)
  (Development|PrintString (Utilities|String|Append "At Login: Spawn location" (Utilities|String|ToString(Transform) SpawnLocation)) true true "(R=0.000000,G=0.658824,B=1.000000,A=1.000000)" 6e+01))
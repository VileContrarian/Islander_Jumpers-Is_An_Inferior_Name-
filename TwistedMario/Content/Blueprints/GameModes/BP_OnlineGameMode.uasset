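; BP_OnlineGameMode is a game mode that spawns and assigns each player's chosen car when play begins.
; The construction script caches BP_GameInfoInstance, which supplies the player count and per-player car selection.
; BeginPlay gathers PlayerStarts, spawns each selected car class at the start with the matching index, and has that index's player controller possess it as a VehicleBase.
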(event EventBeginPlay
  (bind _gameinstanceref (Variables|Default|GetGameInstanceRef))
  (bind _carinforef (Variables|/Game/Blueprints/GameInstances/BP_GameInfoInstance.BP_GameInfoInstance_C|GetCarInfoRef _gameinstanceref))
  (bind _outactors (Actor|GetAllActorsOfClass "/Script/Engine.PlayerStart"))
  (Variables|Default|SetSpawnPoints _outactors)
  (for _index (range 0 (- (Variables|/Game/Blueprints/GameInstances/BP_GameInfoInstance.BP_GameInfoInstance_C|GetMaxPlayerCount (Variables|Default|GetGameInstanceRef)) 1))
    (bind _returnvalue (Game|SpawnActorfromClass (Utilities|Array|Get(acopy) (Variables|/Game/Blueprints/BPD_CarInformation.BPD_CarInformation_C|GetCarClassRef _carinforef) (Utilities|Array|Get(acopy) (Variables|/Game/Blueprints/BPD_CarInformation.BPD_CarInformation_C|GetCarIndex _carinforef) _index)) (Math|Transform|MakeTransform (.location (Transformation|GetActorTransform (Utilities|Array|Get(acopy) (Variables|Default|GetSpawnPoints) _index))) (.rotation (Transformation|GetActorTransform (Utilities|Array|Get(acopy) (Variables|Default|GetSpawnPoints) _index))) "1,1,1") "Undefined" 0 0))
    (bind _asvehicle_base (Utilities|Casting|CastToVehicleBase _returnvalue))
    (Pawn|Possess (Game|GetPlayerController _index) _asvehicle_base)))

(fn ConstructionScript
  (bind _asbp_game_info_instance (Utilities|Casting|CastToBP_GameInfoInstance (Game|GetGameInstance)))
  (Variables|Default|SetGameInstanceRef _asbp_game_info_instance))
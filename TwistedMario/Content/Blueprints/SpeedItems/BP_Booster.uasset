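; BP_Booster is a trigger pickup that gives a BP_VehicleBase01 a temporary speed boost.
; On box overlap it raises the vehicle's max speed to its original value times SpeedMultiplier and scales the CarBody's physics velocity by the same factor for an instant kick.
; After an ActiveTime delay it restores the original max speed and destroys itself, so it remains in the level during the boost.
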(event OnComponentBeginOverlap(BoxTrigger)
  (params (OverlappedComponent :type Primitive%20Component%20Object%20Reference) (OtherActor :type Actor%20Object%20Reference) (OtherComp :type Primitive%20Component%20Object%20Reference) (OtherBodyIndex :type Integer) (bFromSweep :type Boolean) (SweepResult :type Hit%20Result%20Structure%20%28by%20ref%29))
  (bind _asbp_vehicle_base_01 (Utilities|Casting|CastToBP_VehicleBase01 OtherActor))
  (Variables|Default|SetVehicleRef _asbp_vehicle_base_01)
  ;[1 1 1 1 12] Can be set manually if need be
  (bind _output_get (Variables|Default|SetNewSpeedMax (* (Variables|/Script/TwistedMario.VehicleBase|GetspeedMaxOriginal _asbp_vehicle_base_01) (Variables|Default|GetSpeedMultiplier))))
  (Class|VehicleBase|SetSpeedMax _asbp_vehicle_base_01 _output_get)
  (bind _returnvalue (Physics|GetPhysicsLinearVelocity (Variables|/Game/Blueprints/VehicleBase/BP_VehicleBase01.BP_VehicleBase01_C|GetCarBody _asbp_vehicle_base_01) "None"))
  (Physics|SetPhysicsLinearVelocity (Variables|/Game/Blueprints/VehicleBase/BP_VehicleBase01.BP_VehicleBase01_C|GetCarBody _asbp_vehicle_base_01) (* _returnvalue (Variables|Default|GetSpeedMultiplier)) false "None")
  ;[1 1 1 1 12] How long before returning to original max speed?
  (Utilities|FlowControl|Delay (Variables|Default|GetActiveTime))
  (Class|VehicleBase|SetSpeedMax _asbp_vehicle_base_01 (Variables|/Script/TwistedMario.VehicleBase|GetspeedMaxOriginal _asbp_vehicle_base_01))
  ;[1 1 1] Destroy Self
  (Actor|DestroyActor))

(fn ConstructionScript)
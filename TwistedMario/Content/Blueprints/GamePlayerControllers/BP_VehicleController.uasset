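; Player controller for a lap-based vehicle game that drives the possessed BP_VehicleBase01 and tracks per-player stats.
; Movement axes and action inputs are forwarded to the vehicle as acceleration, steering, jump and handbrake.
; Every tick it sets IsFinished by comparing LapIndex with the lap count in BP_GameInfoInstance.
; Helper functions accumulate kills, deaths, damage and healing, while GetRespawnPoint returns a hard-coded transform.
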(event EventTick
  (params (DeltaSeconds :type Float%20%28single-precision%29))
  ;[1 1 1] Event Tick
  (CallFunction|CheckIsFinished))

(event EventBeginPlay
  ;[1 1 1] Begin Play & Setting Input Mode
  (Input|SetInputModeGameOnly self)
  (Variables|Default|SetbShowMouseCursor false))

(event Input|ActionEvents|InputActionPrimary
  (params (Key :type Key%20Structure))
  ;[1 1 1] Input Control If Currently Posessing Pawn
  (:Pressed
    (bind _asbp_vehicle_base_01 (Utilities|Casting|CastToBP_VehicleBase01 (Pawn|GetControlledPawn)))
    (Utilities|IsValid _asbp_vehicle_base_01
      (:Is%20Valid
        (Class|VehicleBase|Jump _asbp_vehicle_base_01)))))

(event Input|ActionEvents|InputActionSecondary
  (params (Key :type Key%20Structure))
  (bind _returnvalue (Pawn|GetControlledPawn))
  ;[1 1 1] Input Control If Currently Posessing Pawn
  (:Pressed
    (bind _asbp_vehicle_base_01 (Utilities|Casting|CastToBP_VehicleBase01 _returnvalue))
    (Utilities|IsValid _asbp_vehicle_base_01
      (:Is%20Valid
        (Class|VehicleBase|HandBrake _asbp_vehicle_base_01))))
  (:Released
    (bind _asbp_vehicle_base_01_2 (Utilities|Casting|CastToBP_VehicleBase01 _returnvalue))
    (Utilities|IsValid _asbp_vehicle_base_01_2
      (:Is%20Valid
        (Class|VehicleBase|ReleaseHandBrake _asbp_vehicle_base_01_2)))))

(event Input|AxisEvents|InputAxisMoveForward
  (params (AxisValue :type Float%20%28single-precision%29))
  ;[1 1 1] Input Control If Currently Posessing Pawn
  (bind _asbp_vehicle_base_01 (Utilities|Casting|CastToBP_VehicleBase01 (Pawn|GetControlledPawn)))
  (Utilities|IsValid _asbp_vehicle_base_01
    (:Is%20Valid
      (Class|VehicleBase|Accelerate _asbp_vehicle_base_01 AxisValue))))

(event Input|AxisEvents|InputAxisMoveSide
  (params (AxisValue :type Float%20%28single-precision%29))
  ;[1 1 1] Input Control If Currently Posessing Pawn
  (bind _asbp_vehicle_base_01 (Utilities|Casting|CastToBP_VehicleBase01 (Pawn|GetControlledPawn)))
  (Utilities|IsValid _asbp_vehicle_base_01
    (:Is%20Valid
      (Class|VehicleBase|Turn _asbp_vehicle_base_01 AxisValue))))

(fn ConstructionScript)

(fn GetRespawnPoint
  (return (Math|Transform|MakeTransform "-250.000000,-4846.679688,100.000000" "0, 0, 0" "1,1,1")))

(fn AddKills
  (Math|Integer|IncrementInt (Variables|Default|GetKillCount)))

(fn AddDeath
  (Math|Integer|IncrementInt (Variables|Default|GetDeathCount)))

(fn AddDamageRecieved
  (params (Amount :type Integer))
  (Variables|Default|SetDamageRecieved (+ Amount (Variables|Default|GetDamageRecieved))))

(fn AddDamageDone
  (params (Amount%20 :type Integer))
  (Variables|Default|SetDamageDone (+ Amount%20 (Variables|Default|GetDamageDone))))

(fn AddHealingDone
  (params (Amount :type Integer))
  (Variables|Default|SetHealingDone (+ Amount (Variables|Default|GetHealingDone))))

(fn CheckIsFinished
  (bind _asbp_game_info_instance (Utilities|Casting|CastToBP_GameInfoInstance (Game|GetGameInstance)))
  (Variables|Default|SetIsFinished (== (Variables|Default|GetLapIndex) (Variables|/Game/Blueprints/GameInstances/BP_GameInfoInstance.BP_GameInfoInstance_C|GetNumberofLaps _asbp_game_info_instance))))
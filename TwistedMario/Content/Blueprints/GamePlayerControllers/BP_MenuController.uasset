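; BP_MenuController is the menu player controller that tracks whether its player is active.
; On BeginPlay it sets Game and UI input and caches BP_MenuGameMode.
; Primary press sets Active if the player is inactive or InPlayerSelect is true, while Secondary clears it only if active and InPlayerSelect is false.
; Both changes call UpdatePlayerCount on the game mode to refresh the player count.
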(event EventBeginPlay
  ;[1 1 1] Begin Play
  (Input|SetInputModeGameandUI self 0 "DoNotLock" false)
  (bind _asbp_menu_game_mode (Utilities|Casting|CastToBP_MenuGameMode (Game|GetGameMode)))
  (Variables|Default|SetMenu%20GameMode _asbp_menu_game_mode))

(event Input|ActionEvents|InputActionPrimary
  (params (Key :type Key%20Structure))
  ;[1 1 1] Check If Player is Active
  (:Pressed
    (if (not (and (Variables|Default|GetActive) (Math|Boolean|NotEqual(Boolean) (Variables|/Game/Blueprints/GameModes/BP_MenuGameMode.BP_MenuGameMode_C|GetInPlayerSelect (Variables|Default|GetMenu%20GameMode)) true)))
      (Variables|Default|SetActive true)
      (Default|UpdatePlayerCount (Variables|Default|GetMenu%20GameMode)))))

(event Input|ActionEvents|InputActionSecondary
  (params (Key :type Key%20Structure))
  ;[1 1 1] Check If Player is Active
  (:Pressed
    (if (and (Variables|Default|GetActive) (Math|Boolean|NotEqual(Boolean) (Variables|/Game/Blueprints/GameModes/BP_MenuGameMode.BP_MenuGameMode_C|GetInPlayerSelect (Variables|Default|GetMenu%20GameMode)) true))
      (Variables|Default|SetActive false)
      (Default|UpdatePlayerCount (Variables|Default|GetMenu%20GameMode)))))

(fn ConstructionScript)
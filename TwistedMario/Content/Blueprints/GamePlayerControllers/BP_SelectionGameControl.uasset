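; Player controller for the car and map selection menus that turns left/right input into list scrolling.
; It caches top-level widgets implementing I_SelectionControl on BeginPlay, with UpdateWidgetList available to refresh that list.
; A/D and left-stick presses set InputDirection and send ScrollThroughListMessage only to active BP_CarSelectionMenu or BP_5_MapSelect widgets.
; HandleCarSelection, not called here, messages just the first cached widget.
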(event Custom|UpdateWidgetList
  (Utilities|Array|Clear (Variables|Default|GetWidgetList))
  (bind _foundwidgets (Class|WidgetBlueprintLibrary|GetAllWidgetswithInterface "/Game/Blueprints/Interfaces/I_SelectionControl.I_SelectionControl_C" true))
  (Variables|Default|SetWidgetList _foundwidgets))

(event EventBeginPlay
  (bind _foundwidgets (Class|WidgetBlueprintLibrary|GetAllWidgetswithInterface "/Game/Blueprints/Interfaces/I_SelectionControl.I_SelectionControl_C" true))
  (Variables|Default|SetWidgetList _foundwidgets))

(event Input|KeyboardEvents|A
  (params (Key :type Key%20Structure))
  (:Pressed
    (Variables|Default|SetInputDirection false)
    (for _array_element (Variables|Default|GetWidgetList)
      (bind _asbp_car_selection_menu (Utilities|Casting|CastToBP_CarSelectionMenu _array_element)
        (:then
          (if (Variables|/Game/UI/BP_CarSelectionMenu.BP_CarSelectionMenu_C|GetwidgetIsActive _asbp_car_selection_menu)
            (Class|ISelectionControl|ScrollThroughList(Message) _array_element (Variables|Default|GetInputDirection))))
        (:CastFailed
          (bind _asbp_5_map_select (Utilities|Casting|CastToBP_5_MapSelect _array_element))
          (if (Variables|/Game/UI/BP_5_MapSelect.BP_5_MapSelect_C|GetwidgetIsActive _asbp_5_map_select)
            (Class|ISelectionControl|ScrollThroughList(Message) _array_element (Variables|Default|GetInputDirection))))))))

(event Input|KeyboardEvents|D
  (params (Key :type Key%20Structure))
  (:Pressed
    (Variables|Default|SetInputDirection true)
    (for _array_element (Variables|Default|GetWidgetList)
      (bind _asbp_car_selection_menu (Utilities|Casting|CastToBP_CarSelectionMenu _array_element)
        (:then
          (if (Variables|/Game/UI/BP_CarSelectionMenu.BP_CarSelectionMenu_C|GetwidgetIsActive _asbp_car_selection_menu)
            (Class|ISelectionControl|ScrollThroughList(Message) _array_element (Variables|Default|GetInputDirection))))
        (:CastFailed
          (bind _asbp_5_map_select (Utilities|Casting|CastToBP_5_MapSelect _array_element))
          (if (Variables|/Game/UI/BP_5_MapSelect.BP_5_MapSelect_C|GetwidgetIsActive _asbp_5_map_select)
            (Class|ISelectionControl|ScrollThroughList(Message) _array_element (Variables|Default|GetInputDirection))))))))

(event Input|GamepadEvents|GamepadLeftStickLeft
  (params (Key :type Key%20Structure))
  (:Pressed
    (Variables|Default|SetInputDirection false)
    (for _array_element (Variables|Default|GetWidgetList)
      (bind _asbp_car_selection_menu (Utilities|Casting|CastToBP_CarSelectionMenu _array_element)
        (:then
          (if (Variables|/Game/UI/BP_CarSelectionMenu.BP_CarSelectionMenu_C|GetwidgetIsActive _asbp_car_selection_menu)
            (Class|ISelectionControl|ScrollThroughList(Message) _array_element (Variables|Default|GetInputDirection))))
        (:CastFailed
          (bind _asbp_5_map_select (Utilities|Casting|CastToBP_5_MapSelect _array_element))
          (if (Variables|/Game/UI/BP_5_MapSelect.BP_5_MapSelect_C|GetwidgetIsActive _asbp_5_map_select)
            (Class|ISelectionControl|ScrollThroughList(Message) _array_element (Variables|Default|GetInputDirection))))))))

(event Input|GamepadEvents|GamepadLeftStickRight
  (params (Key :type Key%20Structure))
  (:Pressed
    (Variables|Default|SetInputDirection true)
    (for _array_element (Variables|Default|GetWidgetList)
      (bind _asbp_car_selection_menu (Utilities|Casting|CastToBP_CarSelectionMenu _array_element)
        (:then
          (if (Variables|/Game/UI/BP_CarSelectionMenu.BP_CarSelectionMenu_C|GetwidgetIsActive _asbp_car_selection_menu)
            (Class|ISelectionControl|ScrollThroughList(Message) _array_element (Variables|Default|GetInputDirection))))
        (:CastFailed
          (bind _asbp_5_map_select (Utilities|Casting|CastToBP_5_MapSelect _array_element))
          (if (Variables|/Game/UI/BP_5_MapSelect.BP_5_MapSelect_C|GetwidgetIsActive _asbp_5_map_select)
            (Class|ISelectionControl|ScrollThroughList(Message) _array_element (Variables|Default|GetInputDirection))))))))

(fn ConstructionScript)

(fn HandleCarSelection
  (for (_array_element _array_index) (Variables|Default|GetWidgetList)
    (if (== _array_index 0)
      (Class|ISelectionControl|ScrollThroughList(Message) _array_element (Variables|Default|GetInputDirection)))))
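; BP_MushroomSpring is a mushroom spring hazard that launches an overlapping BP_VehicleBase01 upward when ready, by adding physics velocity to its car body.
; Tick animates the release as a sine-driven vertical bounce with decaying frequency, then winds the spring down in stepped compressions until it re-arms.
; Dynamic materials on cap and spring fade their intensity during the bounce and ramp it up cubically while winding.
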(event OnComponentBeginOverlap(BoxTrigger)
  (params (OverlappedComponent :type Primitive%20Component%20Object%20Reference) (OtherActor :type Actor%20Object%20Reference) (OtherComp :type Primitive%20Component%20Object%20Reference) (OtherBodyIndex :type Integer) (bFromSweep :type Boolean) (SweepResult :type Hit%20Result%20Structure%20%28by%20ref%29))
  (if (Variables|Default|GetisReady)
    (bind _asbp_vehicle_base_01 (Utilities|Casting|CastToBP_VehicleBase01 OtherActor))
    (Variables|Default|SetVehicleRef _asbp_vehicle_base_01)
    (Variables|Default|SetisSprung true)
    ;[1 1 1] Throw vehicle upward
    (CallFunction|DoPush)))

(event EventBeginPlay
  (Variables|Default|SetInitialScale (Transformation|GetWorldScale (Variables|Default|GetSpring))))

(event EventTick
  (params (DeltaSeconds :type Float%20%28single-precision%29))
  ;[1 1 1 1 15] Charging/Winding Animation
  (CallFunction|DoSpringWind DeltaSeconds)
  ;[1 1 1 1 15] Spring Animation
  (CallFunction|DoSpringUp DeltaSeconds))

(fn ConstructionScript
  (bind _returnvalue (Rendering|Material|CreateDynamicMaterialInstance (Variables|Default|GetCap) 0 "/Game/Materials/0_Arundhati/M_bounceFX.M_bounceFX" "None" :!class /Script/Engine.PrimitiveComponent))
  (Variables|Default|SetCapMaterial _returnvalue)
  (bind _returnvalue_2 (Rendering|Material|CreateDynamicMaterialInstance (Variables|Default|GetSpring) 0 "/Game/Materials/0_Arundhati/M_springFX.M_springFX" "None" :!class /Script/Engine.PrimitiveComponent))
  (Variables|Default|SetSpringMaterial _returnvalue_2))

(fn DoSpringUp
  (params (Time :type Float%20%28single-precision%29%20%28by%20ref%29))
  (bind _spring (Variables|Default|GetSpring))
  (bind _returnvalue (Transformation|GetWorldScale _spring))
  (if (Variables|Default|GetisSprung)
    (bind _output_get (Variables|Default|SetSpringTime (+ Time (stale _output_get))))
    (bind _output_get_2 (Variables|Default|SetSpringSpeed (- (stale _output_get_2) 0.01)))
    (Rendering|Material|SetScalarParameterValue (Variables|Default|GetCapMaterial) "Intensity" (* (- _output_get_2 5.2) 2.0) :!class /Script/Engine.MaterialInstanceDynamic)
    (Rendering|Material|SetScalarParameterValue (Variables|Default|GetSpringMaterial) "Intensity" (/ (* (- _output_get_2 5.2) 2.0) 1.0) :!class /Script/Engine.MaterialInstanceDynamic)
    (Transformation|SetWorldScale3D _spring (Math|Vector|MakeVector (.x _returnvalue) (.y _returnvalue) (* (+ (Math|Float|Absolute(Float) (Math|Trig|Sin(Radians) (* (Variables|Default|GetSpringTime) (Variables|Default|GetSpringSpeed)))) 0.25) (Variables|Default|GetAmplitude))))
    (if (<= (Variables|Default|GetSpringSpeed) 5.2)
      (Variables|Default|SetisSprung false)
      (Variables|Default|SetisReady false)
      (Variables|Default|SetSpringTime 0.0)
      (Variables|Default|SetSpringSpeed (Variables|Default|GetInitialSpringSpeed))
      (Transformation|SetWorldScale3D (Variables|Default|GetSpring) (Variables|Default|GetInitialScale)))))

(fn DoSpringWind
  (params (Time :type Float%20%28single-precision%29%20%28by%20ref%29))
  (bind _spring (Variables|Default|GetSpring))
  (bind _returnvalue (Transformation|GetWorldScale _spring))
  (if (not (Variables|Default|GetisReady))
    (Rendering|Material|SetScalarParameterValue (Variables|Default|GetCapMaterial) "Intensity" (Math|Float|Power (Math|Float|Clamp(Float) (* (Variables|Default|GetWindingTime) 0.3) 0.0 1e+03) 3.0) :!class /Script/Engine.MaterialInstanceDynamic)
    (Rendering|Material|SetScalarParameterValue (Variables|Default|GetSpringMaterial) "Intensity" (Math|Float|Power (Math|Float|Clamp(Float) (* (Variables|Default|GetWindingTime) 0.3) 0.0 1e+03) 3.0) :!class /Script/Engine.MaterialInstanceDynamic)
    (bind _output_get (Variables|Default|SetWindingTime (+ (stale _output_get) Time)))
    (if (== (Math|Integer|%(Integer) (Math|Float|Round _output_get) 2) 0)
      (Transformation|SetWorldScale3D _spring (Math|Vector|MakeVector (.x _returnvalue) (.y _returnvalue) (- (.z _returnvalue) (Variables|Default|GetWindingSpeed))))
      (if (<= (.z (Transformation|GetWorldScale _spring)) 1.5)
        (Variables|Default|SetisReady true)
        (Variables|Default|SetWindingTime 0.0)))))

(fn DoPush
  (Utilities|IsValid (Variables|Default|GetVehicleRef)
    (:Is%20Valid
      (Physics|SetPhysicsLinearVelocity (Variables|/Game/Blueprints/VehicleBase/BP_VehicleBase01.BP_VehicleBase01_C|GetCarBody (Variables|Default|GetVehicleRef)) "0, 0,1000.000000" true "None")
      (Variables|Default|SetVehicleRef 0))))
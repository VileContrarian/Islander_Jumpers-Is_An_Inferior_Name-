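; Windstorm hazard that travels along a spline and pulls in and damages a vehicle caught inside it.
; When active, a timeline moves it along the first SPLINE_Storm found, over a set duration from a start offset.
; InnerCollision overlaps track the vehicle; each Tick, DoVacuum pulls it centerward, fading with horizontal distance and weaker vertically, and damages it.
; StormDamage, which also cuts max speed, is never executed.
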(event OnComponentBeginOverlap(InnerCollision)
  (params (OverlappedComponent :type Primitive%20Component%20Object%20Reference) (OtherActor :type Actor%20Object%20Reference) (OtherComp :type Primitive%20Component%20Object%20Reference) (OtherBodyIndex :type Integer) (bFromSweep :type Boolean) (SweepResult :type Hit%20Result%20Structure%20%28by%20ref%29))
  (bind _asvehicle_base (Utilities|Casting|CastToVehicleBase OtherActor))
  (bind _asbp_vehicle_base_01 (Utilities|Casting|CastToBP_VehicleBase01 _asvehicle_base))
  (Variables|Default|SetInStorm true)
  (Variables|Default|SetVehicle _asbp_vehicle_base_01))

(event OnComponentEndOverlap(InnerCollision)
  (params (OverlappedComponent :type Primitive%20Component%20Object%20Reference) (OtherActor :type Actor%20Object%20Reference) (OtherComp :type Primitive%20Component%20Object%20Reference) (OtherBodyIndex :type Integer))
  (bind _asvehicle_base (Utilities|Casting|CastToVehicleBase OtherActor))
  (bind _asbp_vehicle_base_01 (Utilities|Casting|CastToBP_VehicleBase01 _asvehicle_base))
  (Variables|Default|SetInStorm false)
  (Variables|Default|SetVehicle 0))

(event Custom|MoveStorm
  (Components|Timeline|SetPlayRate (Variables|Default|GetStormPath) (/ 1.0 (Variables|Default|GetDuration)))
  (Components|Timeline|SetNewTime (Variables|Default|GetStormPath) (Variables|Default|GetStartOffset))
  (bind _alpha (Timeline|StormPath Play)
    (:Update
      (Variables|Default|SetAlpha _alpha)
      (Transformation|SetActorLocationAndRotation (Spline|GetLocationatDistanceAlongSpline (Variables|/Game/Blueprints/Splines/SPLINE_Storm.SPLINE_Storm_C|GetStormPath (Variables|Default|GetTrackRef)) (Math|Float|Lerp 0.0 (Spline|GetSplineLength (Variables|/Game/Blueprints/Splines/SPLINE_Storm.SPLINE_Storm_C|GetStormPath (Variables|Default|GetTrackRef))) (Variables|Default|GetAlpha)) "World") (Transformation|GetActorRotation)))))

(event EventBeginPlay
  (if (Variables|Default|GetActiveStorm)
    (bind _outactors (Actor|GetAllActorsOfClass "/Game/Blueprints/Splines/SPLINE_Storm.SPLINE_Storm_C"))
    (bind _asspline_storm (Utilities|Casting|CastToSPLINE_Storm (Utilities|Array|Get(acopy) _outactors)))
    (Variables|Default|SetTrackRef _asspline_storm)
    (CallFunction|MoveStorm)))

(event Collision|EventActorBeginOverlap
  (params (OtherActor :type Actor%20Object%20Reference)))

(event EventTick
  (params (DeltaSeconds :type Float%20%28single-precision%29))
  (bind _vehicle (Variables|Default|GetVehicle))
  (if (Variables|Default|GetInStorm)
    (Utilities|IsValid _vehicle
      (:Is%20Valid
        (CallFunction|DoVacuum _vehicle)))))

(fn ConstructionScript)

(fn StormDamage
  (if (Variables|Default|GetInStorm)
    (bind _asbp_vehicle_base_01 (Utilities|Casting|CastToBP_VehicleBase01 (Game|Player|GetPlayerPawn 0)))
    (Class|VehicleBase|DoDamage _asbp_vehicle_base_01 10)
    ;[1 1 1] If Car's Max Speed is under 120: keep it there. Otherwise Lower It while it's in the Storm
    (if (< (Variables|/Script/TwistedMario.VehicleBase|GetspeedMax _asbp_vehicle_base_01) 1e+02)
      ;[1 1 1] Remove Max Speed, unless it's at 120
      (Variables|/Script/TwistedMario.VehicleBase|SetspeedMax _asbp_vehicle_base_01 1e+02)
      (else
        (Variables|/Script/TwistedMario.VehicleBase|SetspeedMax _asbp_vehicle_base_01 (- (Variables|/Script/TwistedMario.VehicleBase|GetspeedMax _asbp_vehicle_base_01) 1e+01))))))

(fn DoVacuum
  (params (VehicleRef :type BP%20Vehicle%20Base%2001%20Object%20Reference%20%28by%20ref%29))
  (bind _carbody (Variables|/Game/Blueprints/VehicleBase/BP_VehicleBase01.BP_VehicleBase01_C|GetCarBody VehicleRef))
  (bind _innercollision (Variables|Default|GetInnerCollision))
  (bind _maxvacuumforce (Variables|Default|GetMaxVacuumForce))
  (bind _returnvalue (Transformation|GetWorldLocation _carbody))
  (bind _returnvalue_2 (Transformation|GetWorldLocation _innercollision))
  (bind _returnvalue_3 (- _returnvalue_2 _returnvalue))
  (bind _returnvalue_4 (Math|Vector|VectorLength (Math|Vector|MakeVector (.x _returnvalue_3) (.y _returnvalue_3) 0.0)))
  (bind _returnvalue_5 (Math|Float|Clamp(Float) _returnvalue_4 0.0 1e+03))
  (bind _returnvalue_6 (/ _returnvalue_5 1e+03))
  (bind _returnvalue_7 (Math|Float|Lerp _maxvacuumforce 0.0 _returnvalue_6))
  (if (Variables|Default|GetInStorm)
    (Physics|AddForce _carbody (Math|Vector|MakeVector (* (.x _returnvalue_3) _returnvalue_7) (* (.y _returnvalue_3) _returnvalue_7) (/ (* (.z _returnvalue_3) _returnvalue_7) 3.0)) "None" false)
    (Class|VehicleBase|DoDamage VehicleRef 1)))
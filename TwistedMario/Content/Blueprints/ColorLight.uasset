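; An actor Blueprint for a spinning point light that keeps changing color.
; On BeginPlay, a looping one-second timer calls ChangeColor, which converts a random unit vector into a linear color for the PointLight.
; Tick steadily yaws the Light component, scaled by delta time for frame-rate independence.
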(event Custom|Change%20Color
  (Rendering|Components|Light|SetLightColor (Variables|Default|GetPointLight) (Math|Conversions|ToLinearColor(Vector) (Math|Random|RandomUnitVector)) false))

(event EventBeginPlay
  (Utilities|Time|SetTimerbyFunctionName 0 "Change Color" 1.0 true))

(event Collision|EventActorBeginOverlap
  (params (OtherActor :type Actor%20Object%20Reference)))

(event EventTick
  (params (DeltaSeconds :type Float%20%28single-precision%29))
  (Transformation|AddRelativeRotation (Variables|Default|GetLight) (Math|Rotator|MakeRotator 0.0 0.0 (* DeltaSeconds 9.0)) false false))

(fn ConstructionScript)
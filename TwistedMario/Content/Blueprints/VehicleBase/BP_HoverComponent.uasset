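; Hover component that levitates a vehicle's physics mesh above ground from its own location.
; A looping 0.01-second timer, meant to approximate a fixed tick, runs DoLevitation, which traces along the component's down axis.
; Near ground, a falling mesh gets a distance-scaled push along the surface normal; otherwise it gets a constant downward force.
; DoLevitationExperiment holds an alternative spring-damper version, not called in this graph.
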(event Custom|InitComponent
  (params (StaticMesh :type Static%20Mesh%20Component%20Object%20Reference))
  (bind _output_get (Variables|Default|SetCarMesh StaticMesh))
  (Variables|Default|SetMass (Physics|GetMass _output_get)))

(event EventBeginPlay
  ;[1 1 1 1 10] This is a timed loop that manually caps the call cycle of functions run within it. I'm using this to try to get all PC's to simulate similar physics behaviour regardless of their build, since UE doesn't have fixed Tick(). Methods called here are slower and maybe less accurate but generally have the same call rate in any system.
  (Utilities|Time|SetTimerbyFunctionName 0 "DoLevitation" 0.01 true))

(event EventTick
  (params (DeltaSeconds :type Float%20%28single-precision%29)))

(fn DoLevitationExperiment
  (bind _returnvalue (Transformation|GetWorldLocation))
  (bind _carmesh (Variables|Default|GetCarMesh))
  ;[1 1 1] Raycast
  (bind (_outhit _returnvalue_2) (Collision|LineTraceByChannel _returnvalue (+ _returnvalue (* (Math|Vector|GetUpVector) (* (Variables|Default|GetTraceLength) -1.0))) "TraceTypeQuery1" false 0 "None"))
  (if _returnvalue_2
    ;[1 1 1] Check if on the air
    (Variables|Default|SetisHitGround true)
    (else
      (Variables|Default|SetisHitGround false)))
  ;[1 1 1] Hover Method 2
  (bind _output_get (Variables|Default|SetDistanceHit (- (Variables|Default|GetTraceLength) (.Distance (Collision|BreakHitResult _outhit)))))
  ;[1 1 1] Force to Levitate
  (Class|PrimitiveComponent|AddForceatLocation _carmesh (* (* (.ImpactNormal (Collision|BreakHitResult _outhit)) (+ (* (/ (- _output_get (Variables|Default|GetPrevHit)) (Utilities|Time|GetWorldDeltaSeconds)) (Variables|Default|GetDampingCoeff)) (* _output_get (Variables|Default|GetSpringCoeff)))) (Variables|Default|GetHoverForce)) (Transformation|GetWorldLocation) "None")
  ;[1 1 1] Reduce the "wobbling" of the vehicle
  (Class|PrimitiveComponent|SetAngularDamping _carmesh (Variables|Default|GetAngularDamping))
  (Variables|Default|SetPrevHit (Variables|Default|GetDistanceHit)))

(fn DoLevitation
  (bind _returnvalue (Transformation|GetWorldLocation))
  (bind _carmesh (Variables|Default|GetCarMesh))
  (bind (_outhit _returnvalue_2) (Collision|LineTraceByChannel _returnvalue (+ _returnvalue (* (Math|Vector|GetUpVector) (* (Variables|Default|GetTraceLength) -1.0))) "TraceTypeQuery1" false 0 "ForOneFrame"))
  (bind _output_get (Variables|Default|SetisHitGround _returnvalue_2))
  (if _output_get
    (bind _returnvalue_3 (Physics|GetPhysicsLinearVelocity (Variables|Default|GetCarMesh) "None"))
    (if (< (.z _returnvalue_3) 0.0)
      (Class|PrimitiveComponent|AddForceatLocation _carmesh (* (.ImpactNormal (Collision|BreakHitResult _outhit)) (* (Math|Float|Lerp 1e+04 0.0 (/ (.Distance (Collision|BreakHitResult _outhit)) (Variables|Default|GetTraceLength))) (Variables|Default|GetHoverForce))) (Transformation|GetWorldLocation) "None")
      (else
        (Physics|AddForce _carmesh "0, 0,-980.000000" "None" false)))))
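; MainGameMode is a game mode with logic for procedurally building a chain of intermediate road pieces, currently left disconnected.
; BeginPlay, the construction script and the AddIntermediateRoad entry do nothing.
; The unwired loop would spawn ten roads, each supplying the next spawn point from its attach transform, then set EndIntermediate.
; That flag makes the spawner place and register a BP_Teleporter instead, then clear itself.
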(event EventBeginPlay
  ;[1 1 1] Spawn 10 Intermidate Peices
)

(fn ConstructionScript)

(fn AddIntermediateRoad
  ;[1 1 1] Intermediate Spawner
)
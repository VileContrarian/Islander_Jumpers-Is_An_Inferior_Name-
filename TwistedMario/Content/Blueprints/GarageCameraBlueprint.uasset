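; Garage camera Blueprint, apparently intended as a shared view target for up to four local players.
; BeginPlay calls ClassSetup, but that function is empty, so the camera currently does nothing at runtime.
; Its disconnected logic would gather player controllers by index, blend their views to this actor and store them as P1 through P4.
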(event EventBeginPlay
  (CallFunction|ClassSetup))

(fn ConstructionScript)

(fn ClassSetup)
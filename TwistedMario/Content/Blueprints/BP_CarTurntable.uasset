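; Car display turntable that shows a selected car skeletal mesh and spins it continuously.
; On BeginPlay it takes the mesh collection from the game instance's car info and shows the first entry; ChangeSelection swaps meshes by index.
; A looping timer at roughly 60 Hz runs Animate, adding RotationSpeed to the yaw per call and resetting only at exactly 360 degrees.
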(event Custom|ChangeSelection
  (params (CarIndex :type Integer))
  (Class|SkinnedMeshComponent|SetSkeletalMesh (Variables|Default|GetCarModel) (Utilities|Array|Get(acopy) (Variables|Default|GetCarModelRef) CarIndex) true))

(event EventBeginPlay
  (bind _asbp_game_info_instance (Utilities|Casting|CastToBP_GameInfoInstance (Game|GetGameInstance)))
  (Variables|Default|SetGameInstanceRef _asbp_game_info_instance)
  (bind _output_get (Variables|Default|SetCarModelRef (Variables|/Game/Blueprints/BPD_CarInformation.BPD_CarInformation_C|GetCarMeshCollection (Variables|/Game/Blueprints/GameInstances/BP_GameInfoInstance.BP_GameInfoInstance_C|GetCarInfoRef _asbp_game_info_instance))))
  (Class|SkinnedMeshComponent|SetSkeletalMesh (Variables|Default|GetCarModel) (Utilities|Array|Get(acopy) _output_get) true)
  ;[1 1 1] Start Animation / 60 fps?
  (Utilities|Time|SetTimerbyFunctionName 0 "Animate" 0.016667 true))

(fn ConstructionScript)

(fn Animate
  (Transformation|SetRelativeRotation (Variables|Default|GetCarModel) (Math|Rotator|MakeRotator 0.0 0.0 (Variables|Default|GetCurrentRotationAngle)) false false)
  (bind _output_get (Variables|Default|SetCurrentRotationAngle (+ (Variables|Default|GetCurrentRotationAngle) (Variables|Default|GetRotationSpeed))))
  (if (== _output_get 3.6e+02)
    (Variables|Default|SetCurrentRotationAngle 0.0)))